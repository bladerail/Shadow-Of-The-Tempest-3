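; BP_Winch is a winch actor that controls a referenced Portcullis, raising it while a BP_Wizard stands at it.
; Box overlap begin calls Raise on the Portcullis and overlap end calls BeginFall.
; A timeline started at BeginPlay drives two point lights' brightness, while Tick activates Marker only in one specific portcullis state.
; A Rotate function sets the winch's roll, but its only call is in unconnected logic.
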(event `self.ReceiveBeginPlay`
  (bind (_direction _brightness) (`Timeline|Timeline_0` :!via `PlayFromStart`)
    (:`Update`
      (`LightComponent.SetIntensity` (`self.PointLight`) _brightness)
      (`LightComponent.SetIntensity` (`self.PointLight1`) _brightness))))

(event `self.ReceiveTick`
  (params (DeltaSeconds :type "Float (single-precision)"))
  (bind _marker (`self.Marker`))
  (if (`|EnumEquality` (`/Game/Props/BP_Doorway.CurrentState` (`self.Portcullis`)) "NewEnumerator1")
    (`ActorComponent.SetActive` _marker true false)
    (else
      (`ActorComponent.SetActive` _marker false false))))

(event `self.Box.OnComponentBeginOverlap`
  (params (OverlappedComponent :type "PrimitiveComponent Object Reference") (OtherActor :type "Actor Object Reference") (OtherComp :type "PrimitiveComponent Object Reference") (OtherBodyIndex :type Integer) (bFromSweep :type Boolean) (SweepResult :type "HitResult Structure (by ref)"))
  (cast `/Game/Players/BP_Wizard` OtherActor)
  (`/Game/Props/BP_Doorway.Raise` (`self.Portcullis`)))

(event `self.Box.OnComponentEndOverlap`
  (params (OverlappedComponent :type "PrimitiveComponent Object Reference") (OtherActor :type "Actor Object Reference") (OtherComp :type "PrimitiveComponent Object Reference") (OtherBodyIndex :type Integer))
  (cast `/Game/Players/BP_Wizard` OtherActor)
  (`/Game/Props/BP_Doorway.BeginFall` (`self.Portcullis`)))

(fn `Rotate`
  (params (Degrees :type "Float (double-precision)"))
  (bind _winch (`self.Winch`))
  (bind (_relativerotation_roll _relativerotation_pitch _relativerotation_yaw) (`KismetMathLibrary.BreakRotator` (`SceneComponent.RelativeRotation` _winch)))
  (`SceneComponent.K2_SetRelativeRotation` _winch (`KismetMathLibrary.MakeRotator` Degrees _relativerotation_pitch _relativerotation_yaw) false false))

(fn `UserConstructionScript`)