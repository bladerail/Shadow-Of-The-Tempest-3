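; BP_Torch is a torch actor for the medieval dungeon, with a fire effect and a point light that can be switched on and off.
; TurnOnTorch and TurnOffTorch toggle the PTorchFire component's active state and the TorchPointLight's visibility together.
; GetPointLightSource exposes the point light to callers.
; The event graph and construction script hold no logic, so any switching comes from calls to these functions.
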(event `self.ReceiveBeginPlay`)

(fn `GetPointLightSource`
  (returns (PointLightObj :type "PointLightComponent Object Reference"))
  (return (`self.Torch_PointLight`)))

(fn `TurnOffTorch`
  (`ActorComponent.SetActive` (`self.P_Torch_Fire`) false false)
  (`SceneComponent.SetVisibility` (`self.Torch_PointLight`) false false))

(fn `TurnOnTorch`
  (`ActorComponent.SetActive` (`self.P_Torch_Fire`) true false)
  (`SceneComponent.SetVisibility` (`self.Torch_PointLight`) true false))

(fn `UserConstructionScript`)