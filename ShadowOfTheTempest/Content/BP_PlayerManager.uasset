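; Manager actor that tracks two-player progress through waypoints, steering two wisps and switching music.
; After a short delay, a looping timer advances the current waypoint to the next later one containing either player, never backwards.
; Each tick of that timer moves the wisps to the waypoint's targets and plays its sounds.
; It plays level music until the last waypoint, then boss music, and triggers victory music once BP_Boss1's health is depleted.
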(event `self.ReceiveBeginPlay`
  (`AudioComponent.Stop` (`self.Boss`))
  (`AudioComponent.Stop` (`self.Level`))
  (`AudioComponent.Stop` (`self.Victory`))
  (`KismetSystemLibrary.Delay` 2.0)
  (`KismetSystemLibrary.K2_SetTimer` null "RecurringFunction" (`self.RecurringTime`) true))

(fn `RecurringFunction`
  (bind _waypoints (`self.Waypoints`))
  (bind _boss (`self.Boss`))
  (bind _level (`self.Level`))
  (bind _currentwaypoint (`self.CurrentWayPoint`))
  (bind _output (`|GetArrayItem` _waypoints _currentwaypoint))
  (bind _sound1 (`/Game/BP_Waypoint.Sound1` _output))
  (bind _sound2 (`/Game/BP_Waypoint.Sound2` _output))
  (bind _wisp1loc (`/Game/BP_Waypoint.Wisp1Loc` _output))
  (bind _wisp2loc (`/Game/BP_Waypoint.Wisp2Loc` _output))
  (for (_array_element _array_index) _waypoints
    (if (> _array_index (`self.CurrentWayPoint`))
      (bind _inside (`/Game/BP_Waypoint.IsPlayerInside` _array_element 0))
      (bind _inside_2 (`/Game/BP_Waypoint.IsPlayerInside` _array_element 1))
      (if (or _inside _inside_2)
        (set `self.CurrentWayPoint` _array_index)
        (break))))
  (`|ExecutionSequence`
    (:`then_0`
      (if (`KismetSystemLibrary.IsValid` _wisp1loc)
        (`/Game/BP_Wisp.Move` (`self.Wisp1`) (`self.K2_GetActorLocation` _wisp1loc))))
    (:`then_1`
      (if (`KismetSystemLibrary.IsValid` _wisp2loc)
        (`/Game/BP_Wisp.Move` (`self.Wisp2`) (`self.K2_GetActorLocation` _wisp2loc))))
    (:`then_2`
      (if (`KismetSystemLibrary.IsValid` _sound1)
        (`GameplayStatics.PlaySound2D` (`self.Wisp1`) _sound1 1.0 1.0 0.0 null null)))
    (:`then_3`
      (if (`KismetSystemLibrary.IsValid` _sound2)
        (`GameplayStatics.PlaySound2D` (`self.Wisp2`) _sound2 1.0 1.0 0.0 null null)))
    (:`then_4`
      (if (== (- _currentwaypoint -1) (`KismetArrayLibrary.Array_Length` (`self.Waypoints`)))
        (if (not (`AudioComponent.IsPlaying` _boss))
          (`AudioComponent.Play` _boss 0.0)
          (`AudioComponent.Stop` (`self.Level`)))
        (elif (not (`AudioComponent.IsPlaying` _level))
          (`AudioComponent.Play` _level 0.0)
          (`AudioComponent.Stop` (`self.Boss`)))))
    (:`then_5`
      (bind _outactors (`GameplayStatics.GetAllActorsOfClass` "/Game/Enemies/BP_Boss1.BP_Boss1_C"))
      (if (<= (`/Game/Enemies/BP_GenericEnemy.Health` (`|GetArrayItem` _outactors)) 0)
        (`AudioComponent.Stop` (`self.Boss`))
        (`AudioComponent.Play` (`self.Victory`) 0.0)))))

(fn `SetWispStart`)

(fn `UserConstructionScript`)