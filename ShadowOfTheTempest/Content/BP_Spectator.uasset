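; Spectator pawn that flies the player's view around with movement and look input, on either a flat screen or a VR headset.
; On BeginPlay it locks the camera to an enabled HMD with eye-level tracking, adding controller roll for PSVR, or otherwise uses control rotation.
; Movement follows the camera's forward and right vectors, while turn and look have direct and frame-time-scaled rate axes.
; A Quit action exits the game.
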(event `self.ReceiveBeginPlay`
  (bind _camera (`self.Camera`))
  ;[1 1 1] Set HMD and controllers
  (`|ExecutionSequence`
    (:`then_0`
      (if (`HeadMountedDisplayFunctionLibrary.IsHeadMountedDisplayEnabled`)
        (set `CameraComponent.bLockToHmd` true _camera)
        (set `CameraComponent.bUsePawnControlRotation` false _camera)
        (switch `name` (`HeadMountedDisplayFunctionLibrary.GetHMDDeviceName`)
          (:`Oculus HMD`
            (`HeadMountedDisplayFunctionLibrary.SetTrackingOrigin` "Eye" :!label _label))
          (:`SteamVR`
            (goto _label))
          (:`PSVR`
            (`HeadMountedDisplayFunctionLibrary.SetTrackingOrigin` "Eye")
            (set `self.bUseControllerRotationRoll` true)))
        (else
          (set `CameraComponent.bLockToHmd` false _camera)
          (set `CameraComponent.bUsePawnControlRotation` true _camera))))
    (:`then_1`)))

(event `InputAction|Quit`
  (params (Key :type "Key Structure"))
  ;[1 1 1] Set HMD and controllers
  (:`Pressed`
    (`KismetSystemLibrary.QuitGame` null "Quit")))

(event `InputAxis|MoveForward`
  (params (AxisValue :type "Float (single-precision)"))
  ;[1 1 1] Set HMD and controllers
  (`self.AddMovementInput` (`SceneComponent.GetForwardVector` (`self.Camera`)) AxisValue))

(event `InputAxis|MoveRight`
  (params (AxisValue :type "Float (single-precision)"))
  ;[1 1 1] Set HMD and controllers
  (`self.AddMovementInput` (`SceneComponent.GetRightVector` (`self.Camera`)) AxisValue))

(event `InputAxis|Turn`
  (params (AxisValue :type "Float (single-precision)"))
  (`self.AddControllerYawInput` AxisValue))

(event `InputAxis|LookUp`
  (params (AxisValue :type "Float (single-precision)"))
  (`self.AddControllerPitchInput` AxisValue))

(event `InputAxis|TurnRate`
  (params (AxisValue :type "Float (single-precision)"))
  (`self.AddControllerYawInput` (* AxisValue (`self.BaseTurnRate`) (`GameplayStatics.GetWorldDeltaSeconds`))))

(event `InputAxis|LookUpRate`
  (params (AxisValue :type "Float (single-precision)"))
  (`self.AddControllerPitchInput` (* AxisValue (`self.BaseLookUpRate`) (`GameplayStatics.GetWorldDeltaSeconds`))))

(fn `UserConstructionScript`)