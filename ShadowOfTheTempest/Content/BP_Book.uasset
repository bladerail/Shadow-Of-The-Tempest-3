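; Animated book actor that opens and closes in an endless loop, bobbing vertically on a cosine wave while open.
; Open rotates the front cover with a timeline, then a second timeline ramps up a point light and progressively spawns page meshes.
; Each page gets a dynamic material with flip and staggered flip-delay parameters, so the material handles page turning.
; Close destroys the pages, switches off the light and plays a cover timeline in reverse.
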(event `self.ReceiveBeginPlay`
  (set `self.Start` (`self.K2_GetActorLocation`))
  (set `self.StartRotation` (`KismetMathLibrary.Conv_RotatorToVector` (`SceneComponent.K2_GetComponentRotation` (`self.Book_Front`))))
  (`self.Open` :!label _label)
  (`KismetSystemLibrary.Delay` 3.0)
  (`self.Close`)
  (`KismetSystemLibrary.Delay` 3.0)
  (goto _label))

(event `self.ReceiveTick`
  (params (DeltaSeconds :type "Float (single-precision)"))
  (bind (_start_x _start_y _start_z) (`KismetMathLibrary.BreakVector` (`self.Start`)))
  (if (`self.Active`)
    (bind _output_get (set `self.FloatTime` (+ DeltaSeconds (`self.FloatTime`))))
    (`self.K2_SetActorLocation` (`KismetMathLibrary.MakeVector` _start_x _start_y (+ (* (- 1.0 (`KismetMathLibrary.Cos` _output_get)) (`self.Float Variance`)) _start_z)))))

(event `Open`
  (bind (_startrotation_x _startrotation_y _startrotation_z) (`KismetMathLibrary.BreakVector` (`self.StartRotation`)))
  (bind _current_page (`self.Current_Page`))
  (if (not (`self.Active`))
    (set `self.Active` true)
    ;[1 1 1] Open book
    (bind (_direction _newtrack_0) (`Timeline|Timeline_1` :!via `PlayFromStart`)
      (:`Update`
        (`SceneComponent.K2_SetWorldRotation` (`self.Book_Front`) (`KismetMathLibrary.MakeRotator` (+ _startrotation_x (* _newtrack_0 -180.0)) _startrotation_y _startrotation_z) false false))
      (:`Finished`
        (set `self.Current_Page` 0)
        (bind (_direction_2 _newtrack_0_2) (`Timeline|Timeline_0` :!via `PlayFromStart`)
          (:`Update`
            (`LightComponent.SetIntensity` (`self.PointLight`) (* _newtrack_0_2 (`self.Max Intensity`)))
            (if (>= (- (* (`self.Pages`) _newtrack_0_2) (`KismetMathLibrary.Conv_IntToDouble` _current_page)) 0.0)
              (bind _returnvalue (`AddComponent|NODE_AddStaticMeshComponent-1` :`RelativeTransform` (`SceneComponent.GetRelativeTransform` (`self.Page_Root`))))
              (`KismetArrayLibrary.Array_Add` (`self.PageMesh`) _returnvalue)
              (`StaticMeshComponent.SetStaticMesh` _returnvalue "/Game/paper_1d.paper_1d")
              (bind _returnvalue_2 (`PrimitiveComponent.CreateDynamicMaterialInstance` _returnvalue 0 "/Game/M_book.M_book" "None"))
              (`MaterialInstanceDynamic.SetScalarParameterValue` _returnvalue_2 "Flip" 1.0)
              (`MaterialInstanceDynamic.SetScalarParameterValue` _returnvalue_2 "Flip delay" (/ _newtrack_0_2 2.0))
              (set `self.Current_Page` (+ _current_page 1)))))))))

(event `Close`
  (bind _pagemesh (`self.PageMesh`))
  (bind (_startrotation_x _startrotation_y _startrotation_z) (`KismetMathLibrary.BreakVector` (`self.StartRotation`)))
  (set `self.Active` false)
  (for _array_element _pagemesh
    (`ActorComponent.K2_DestroyComponent` _array_element))
  (`KismetArrayLibrary.Array_Clear` _pagemesh)
  (`LightComponent.SetIntensity` (`self.PointLight`) 0.0)
  ;[1 1 1] Open book
  (bind (_direction _newtrack_0) (`Timeline|Timeline_2` :!via `ReverseFromEnd`)
    (:`Update`
      (`SceneComponent.K2_SetWorldRotation` (`self.Book_Front`) (`KismetMathLibrary.MakeRotator` (+ _startrotation_x (* _newtrack_0 -180.0)) _startrotation_y _startrotation_z) false false))))

(fn `UserConstructionScript`)