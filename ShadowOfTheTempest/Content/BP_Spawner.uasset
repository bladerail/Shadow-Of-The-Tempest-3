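; Ambush spawner that activates a preset list of Enemies when a BP_Wizard enters its Box trigger.
; BeginPlay turns off their tick and collision through EnableActor.
; While Active, an overlap prints "Ambush!", waits for Delay, then re-enables them and sets each one's Active flag.
; EnableActor feeds its flag straight into SetActorHiddenInGame, so enemies start visible and become hidden on activation.
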(event `self.ReceiveBeginPlay`
  (for _array_element (`self.Enemies`)
    (`self.EnableActor` _array_element)))

(event `self.Box.OnComponentBeginOverlap`
  (params (OverlappedComponent :type "PrimitiveComponent Object Reference") (OtherActor :type "Actor Object Reference") (OtherComp :type "PrimitiveComponent Object Reference") (OtherBodyIndex :type Integer) (bFromSweep :type Boolean) (SweepResult :type "HitResult Structure (by ref)"))
  (if (`self.Active`)
    (cast `/Game/Players/BP_Wizard` OtherActor)
    (`KismetSystemLibrary.PrintString` "Ambush!")
    (`KismetSystemLibrary.Delay` (`self.Delay`))
    (for _array_element (`self.Enemies`)
      (`self.EnableActor` _array_element true)
      (set `/Game/Enemies/BP_GenericEnemy.Active` true _array_element))))

(fn `EnableActor`
  (params (Actor :type "Actor Object Reference") (Active :type Boolean))
  (`self.SetActorHiddenInGame` Actor Active)
  (`self.SetActorTickEnabled` Actor Active)
  (`self.SetActorEnableCollision` Actor Active))

(fn `UserConstructionScript`)