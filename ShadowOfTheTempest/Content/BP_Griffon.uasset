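; Griffon enemy actor that fires projectiles and reacts to projectile hits.
; On overlap, if OnHit returns false and Mode is not 2, a BP_SimpleProjectile triggers the damage animation and is destroyed.
; AttackEffect spawns a BP_EnemyProjectile slightly above the actor along its rotation, and ServerDestroyApparition destroys a given target.
; BeginPlay, Tick, Loop and the construction script are empty.
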(event `self.ReceiveActorBeginOverlap`
  (params (OtherActor :type "Actor Object Reference"))
  (bind _shouldnotplayanim (`self.OnHit` OtherActor))
  (if (not _shouldnotplayanim)
    (bind _asbp_simple_projectile (cast `/Game/Players/BP_SimpleProjectile` OtherActor))
    (if (not (== (`self.Mode`) 2))
      (`SkeletalMeshComponent.PlayAnimation` (`self.Mesh`) "/Game/Enemies/Apparition/Animation/Apparition_Damage_Anim.Apparition_Damage_Anim" false)
      (`self.K2_DestroyActor` _asbp_simple_projectile))))

(event `self.AttackEffect`
  (`|SpawnActorFromClass` "/Game/Enemies/BP_EnemyProjectile.BP_EnemyProjectile_C" (`KismetMathLibrary.MakeTransform` (+ (`self.K2_GetActorLocation`) (0.0 0.0 50.0)) (`self.K2_GetActorRotation`)) "Undefined" "OverrideRootScale" null null))

(event `Server Destroy Apparition`
  (params (`Destroy Target` :type "Actor Object Reference"))
  (`self.K2_DestroyActor` `Destroy Target`))

(fn `Loop`)

(fn `UserConstructionScript`)