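; Scripts a two-player boss encounter, with Start bringing in the boss and Separate running a mid-fight cutscene.
; Separate enables the spawner, hands player controllers to cine pawns, and lets borrowed AI controllers walk the characters onward.
; Chained AI moves and timelines sequence the boss attack, waterfalls, debris, bridge height and rising water.
; Control then returns to players as the boss arcs to its next position and reactivates.
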(event `self.ReceiveBeginPlay`
  (`AudioComponent.Stop` (`self.Audio`))
  (`AudioComponent.Stop` (`self.Audio1`))
  (`AudioComponent.Stop` (`self.Audio2`))
  (`AudioComponent.Stop` (`self.Audio3`))
  (for _array_element (`self.Waterfall`)
    (`ActorComponent.Deactivate` (`Emitter.ParticleSystemComponent` _array_element))
    (set `self.AIController1` (`Pawn.GetController` (`self.AI1`)))
    (set `self.AIController2` (`Pawn.GetController` (`self.AI2`)))))

(event `Start`
  (bind _boss (`self.Boss`))
  (if (not (`self.Started`))
    (set `self.Started` true)
    (`|AIMoveTo` _boss (`self.K2_GetActorLocation`) null 20.0
      (:`OnSuccess`
        (`AudioComponent.Play` (`self.Audio2`) 0.0)
        (`KismetSystemLibrary.Delay` 5.0)
        (if (not (`self.Separated`))
          (`/Game/Enemies/BP_GenericEnemy.SetActive` _boss true))))))

(event `Separate`
  (bind _boss (`self.Boss`))
  (bind _marker (`self.Marker`))
  (bind _boss_2 (`self.Boss`))
  (bind _p1_next (`self.P1_next`))
  (bind _p2_next (`self.P2_next`))
  (bind _marker_2 (`self.Marker`))
  (bind _debris (`self.Debris`))
  (bind (_returnvalue_x _returnvalue_y) (`KismetMathLibrary.BreakVector` (`self.K2_GetActorLocation` (`self.Bridge`))))
  (bind (_returnvalue_x_2 _returnvalue_y_2) (`KismetMathLibrary.BreakVector` (`self.K2_GetActorLocation` _debris)))
  (bind (_returnvalue_x_3 _returnvalue_y_3) (`KismetMathLibrary.BreakVector` (`self.K2_GetActorLocation` (`self.BossNext`))))
  (set `/Game/BP_Spawner.Active` true (`self.Spawner`))
  (if (not (`self.Separated`))
    (set `self.Separated` true)
    (`self.ChangeToCine` (`self.Boss`))
    (`|AIMoveTo` _boss (`self.K2_GetActorLocation`) self 20.0
      (:`OnSuccess`
        _)
      (:`OnFail`
        _))
    (`|AIMoveTo` _boss (`self.K2_GetActorLocation` _marker) _marker 100.0
      (:`OnSuccess`
        _)
      (:`OnFail`
        _))
    (`/Game/Enemies/BP_GenericEnemy.Attack` _boss_2 _marker_2)
    (`AudioComponent.Play` (`self.Audio1`) 0.0)
    (`/Game/Enemies/BP_GenericEnemy.Attack` _boss_2 _marker_2)
    (`AudioComponent.Play` (`self.Audio3`) 0.0)
    (for _array_element (`self.Waterfall`)
      (`ActorComponent.Activate` (`Emitter.ParticleSystemComponent` _array_element) true))
    (`KismetSystemLibrary.Delay` 2.0)
    (`/Game/Enemies/BP_GenericEnemy.StopAttack` _boss_2)
    (`|AIMoveTo` (`self.Player1`) (`self.K2_GetActorLocation` _p1_next) _p1_next 20.0
      (:`then`
        (`|AIMoveTo` (`self.Player2`) (`self.K2_GetActorLocation` _p2_next) _p2_next 20.0
          (:`then`
            (`self.K2_SetActorRotation` (`self.Boss`) (`KismetMathLibrary.FindLookAtRotation` (`self.K2_GetActorLocation`) (`self.K2_GetActorLocation` (`self.BossNext`))) false)
            (`KismetSystemLibrary.PrintString` "Hello")
            (bind (_direction _height) (`Timeline|Timeline_0` :!via `PlayFromStart`)
              (:`Update`
                (`self.K2_SetActorLocation` _debris (`KismetMathLibrary.MakeVector` _returnvalue_x_2 _returnvalue_y_2 _height) false false))
              (:`Finished`
                (bind (_direction_2 _height_2) (`Timeline|Timeline_1` :!via `ReverseFromEnd`)
                  (:`Update`
                    (`self.K2_SetActorLocation` (`KismetMathLibrary.MakeVector` _returnvalue_x _returnvalue_y _height_2)))
                  (:`Finished`
                    (`/Game/Players/Spells/BP_Water.Raise` (`self.Water`))
                    (`KismetSystemLibrary.Delay` 2.0)
                    (`self.ChangeToPlayer`)
                    (bind _output_get (set `self.BossPos` (`self.K2_GetActorLocation` (`self.Boss`))))
                    (bind (_direction_3 _newtrack_0 _newtrack_1) (`Timeline|Timeline_2` :!via `PlayFromStart`)
                      (:`Update`
                        (bind (_returnvalue_x_4 _returnvalue_y_4) (`KismetMathLibrary.BreakVector` (`KismetMathLibrary.VLerp` (`KismetMathLibrary.MakeVector` (.x _output_get) (.y _output_get)) (`KismetMathLibrary.MakeVector` _returnvalue_x_3 _returnvalue_y_3) _newtrack_1)))
                        (`self.K2_SetActorLocation` (`self.Boss`) (`KismetMathLibrary.MakeVector` _returnvalue_x_4 _returnvalue_y_4 (+ (.z _output_get) (* _newtrack_0 500.0))) false false))
                      (:`Finished`
                        (set `/Game/Enemies/BP_GenericEnemy.Active` true (`self.Boss`))
                        (`AudioComponent.Play` (`self.Audio`) 0.0)))))))))))))

(fn `ChangeToCine`
  (params (self2 :type "/Game/Enemies/BP_GenericEnemy Object Reference"))
  (bind _returnvalue (`GameplayStatics.GetPlayerController` 0))
  (bind _returnvalue_2 (`GameplayStatics.GetPlayerController` 1))
  (`/Game/Enemies/BP_GenericEnemy.SetActive` self2 false)
  (bind _output_get (set `self.Player1` (`Controller.K2_GetPawn` _returnvalue)))
  (bind _output_get_2 (set `self.Player2` (`Controller.K2_GetPawn` _returnvalue_2)))
  (`Controller.Possess` _returnvalue (`self.Cine1`))
  (`Controller.Possess` _returnvalue_2 (`self.Cine2`))
  (`Controller.Possess` (`self.AIController1`) _output_get)
  (`Controller.Possess` (`self.AIController2`) _output_get_2))

(fn `ChangeToPlayer`
  (`Controller.Possess` (`GameplayStatics.GetPlayerController` 0) (`self.Player1`))
  (`Controller.Possess` (`GameplayStatics.GetPlayerController` 1) (`self.Player2`)))

(fn `UserConstructionScript`)