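; Debug variant of the Shadow Wizard player, who casts a platform spell only while in shadow.
; A looping timer line-traces to point, directional and rect lights and BPI_LightTrace actors, setting IsInShadow one pass late and updating debug text.
; Fire spawns a platform beyond the targeted stone pillar, facing away from the caster and scaled by pillar bounds.
; Test inputs toggle shadow state, spawn projectiles and show an enemy health bar.
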(event `Key|Two`
  (params (Key :type "Key Structure"))
  (bind _projspawnpoint (`self.ProjSpawnPoint`))
  ;[1 1 1] Proj1test
  (:`Pressed`
    (`|SpawnActorFromClass` "/Game/Players/Spells/Projectiles/BP_ProjBase.BP_ProjBase_C" (`KismetMathLibrary.MakeTransform` (`SceneComponent.K2_GetComponentLocation` _projspawnpoint) (`SceneComponent.K2_GetComponentRotation` _projspawnpoint)) "Undefined" "OverrideRootScale" null null :!label _label)
    (`KismetSystemLibrary.PrintString` "Hello")))

(event `Key|One`
  (params (Key :type "Key Structure"))
  ;[1 1 1] Proj1test
  (:`Pressed`
    (goto _label)))

(event `self.ReceiveBeginPlay`
  (`KismetSystemLibrary.Delay` (`self.ShadowTestFreq`) :!label _label_2)
  (`self.UpdateInShadow`)
  (`self.Debug_ShowInShadow`)
  (goto _label_2))

(event `InputAction|Fire`
  (params (Key :type "Key Structure"))
  (:`Pressed`
    (if (`self.IsInShadow`)
      (bind _actor (`self.GetTarget`))
      (bind _asbp_stone_pillar (cast `/Game/Players/Spells/BP_StonePillar` _actor))
      (`self.CastProjectPlatformSpell` (`self.K2_GetActorLocation`) _asbp_stone_pillar))))

(event `InputAction|Aim`
  (params (Key :type "Key Structure"))
  (:`Pressed`
    (bind _isa (`/Engine/EditorBlueprintResources/StandardMacros.FlipFlop`)
      (:`A`
        _)
      (:`B`
        _))
    (bind _output_get (set `self.IsInShadow` (not _isa)))
    (`KismetSystemLibrary.PrintString` (`KismetStringLibrary.Conv_BoolToString` _output_get))))

(event `Key|Two`
  (params (Key :type "Key Structure"))
  (:`Pressed`
    (bind _returnvalue (`|CreateWidget` "/Game/Players/HPBar/Widget_EnemyHealthBar.Widget_EnemyHealthBar_C"))
    (`UserWidget.AddToViewport` _returnvalue 0)))

(event `self.SetNewActiveSpell`
  (params (NewSpellActor :type "Actor Object Reference"))
  (if (== null null)
    _
    (elif (not (== (`self.ActiveSpellOnMap`) null))
      (`self.K2_DestroyActor` (`self.ActiveSpellOnMap`))))
  (set `self.ActiveSpellOnMap` null))

(fn `CastProjectPlatformSpell`
  (params (CastPoint :type "Vector Structure") (TargetPillar :type "Actor Object Reference"))
  (locals (LTargetPillar :type "Actor Object Reference") (LDirection :type "Vector Structure") (LPillarHeight :type "Float (double-precision)"))
  (bind (_origin _boxextent) (`self.GetActorBounds` (`local.LTargetPillar`) false))
  (bind _output_get (set `local.LTargetPillar` TargetPillar))
  (bind _output_get_2 (set `local.LDirection` (- (`KismetMathLibrary.MakeVector` (.x (`self.K2_GetActorLocation` _output_get)) (.y (`self.K2_GetActorLocation` _output_get))) (`KismetMathLibrary.MakeVector` (.x CastPoint) (.y CastPoint)))))
  (bind _output_get_3 (set `local.LPillarHeight` (.z _boxextent)))
  (`|SpawnActorFromClass` "/Game/Players/Spells/BP_Platform.BP_Platform_C" (`KismetMathLibrary.MakeTransform` (+ _output_get_2 (`self.K2_GetActorLocation` (`local.LTargetPillar`))) (`KismetMathLibrary.MakeRotFromX` (`local.LDirection`)) (`KismetMathLibrary.MakeVector` (/ _output_get_3 50.0) (/ (.y _boxextent) 100.0) 1.0)) "Undefined" "OverrideRootScale" null null)
  (`self.SetNewActiveSpell` null))

(fn `Debug_ShowInShadow`
  (bind _dbg_inshadow (`self.DBG_Inshadow`))
  (if (`self.IsInShadow`)
    (`TextRenderComponent.K2_SetText` _dbg_inshadow (`self.DBG_InshadowStr`))
    (else
      (`TextRenderComponent.K2_SetText` _dbg_inshadow (`self.DBG_NotinshadowStr`)))))

(fn `HitBySpell`
  (params (Damage :type "Float (double-precision)"))
  (returns (qqq :type Boolean))
  (return false))

(fn `UpdateInShadow`
  (bind _returnvalue (`SceneComponent.K2_GetComponentLocation` (`self.CapsuleComponent`)))
  ;[1 1 1] UE4 built in Light
  (set `self.IsInShadow` (not (`self.Tempvar_islighted`)))
  (set `self.Tempvar_islighted` false)
  (bind _outactors (`GameplayStatics.GetAllActorsOfClass` "/Script/Engine.PointLight"))
  (for _array_element _outactors
    (bind (_outhit _returnvalue_2) (`KismetSystemLibrary.LineTraceSingle` (`SceneComponent.K2_GetComponentLocation` (`self.CapsuleComponent`)) (`SceneComponent.K2_GetComponentLocation` (`Actor.RootComponent` _array_element)) "TraceTypeQuery1"))
    (if (not _returnvalue_2)
      (set `self.Tempvar_islighted` true)))
  (bind _outactors_2 (`GameplayStatics.GetAllActorsOfClass` "/Script/Engine.DirectionalLight"))
  (for _array_element_2 _outactors_2
    (bind (_outhit_2 _returnvalue_3) (`KismetSystemLibrary.LineTraceSingle` _returnvalue (+ (* (`KismetMathLibrary.GetForwardVector` (`SceneComponent.K2_GetComponentRotation` (`Light.LightComponent` _array_element_2))) -10000.0) _returnvalue) "TraceTypeQuery1"))
    (if (not _returnvalue_3)
      (set `self.Tempvar_islighted` true)))
  (bind _outactors_3 (`GameplayStatics.GetAllActorsOfClass` "/Script/Engine.RectLight"))
  (for _array_element_3 _outactors_3
    (bind (_outhit_3 _returnvalue_4) (`KismetSystemLibrary.LineTraceSingle` (`SceneComponent.K2_GetComponentLocation` (`self.CapsuleComponent`)) (`SceneComponent.K2_GetComponentLocation` (`Actor.RootComponent` _array_element_3)) "TraceTypeQuery1"))
    (if (not _returnvalue_4)
      (set `self.Tempvar_islighted` true)))
  (bind _outactors_4 (`GameplayStatics.GetAllActorsWithInterface` "/Game/Players/LightTrace/BPI_LightTrace.BPI_LightTrace_C"))
  (for _array_element_4 _outactors_4
    (bind _pointlightobj (message `/Game/Players/LightTrace/BPI_LightTrace.GetPointLightSource` _array_element_4))
    (bind (_outhit_4 _returnvalue_5) (`KismetSystemLibrary.LineTraceSingle` (`SceneComponent.K2_GetComponentLocation` (`self.CapsuleComponent`)) (`SceneComponent.K2_GetComponentLocation` _pointlightobj) "TraceTypeQuery1"))
    (if (not _returnvalue_5)
      (set `self.Tempvar_islighted` true))))

(fn `UserConstructionScript`)