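; BP_RuneBox is a physics cube that gets pushed when a spell is cast on it.
; On CastSpell, GetNearestSocket finds the cube socket closest to the contact point, and an impulse scaled by spell strength is applied there toward the cube's center.
; A rune-push particle facing the cast point spawns on that socket, along with a wind sound.
; AddForceFuncOld, an older continuous-force approach, remains but is never called.
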(event `self.ReceiveTick`
  (params (DeltaSeconds :type "Float (single-precision)")))

(event `/Game/Players/Spells/BP_Spell_Interface.CastSpell`
  (params (CastPoint :type "Vector Structure") (Strength :type "Float (single-precision)") (ContactPoint :type "Vector Structure"))
  (bind _cube (`self.Cube`))
  (bind (_nearest_socket_name _nearest_socket_location) (`self.GetNearestSocket` ContactPoint))
  (bind _output_get (set `self.Delta Strength` (* Strength 5000.0)))
  (bind _output_get_2 (set `self.ForceDirection` (`KismetMathLibrary.GetDirectionUnitVector` _nearest_socket_location (`SceneComponent.K2_GetComponentLocation` (`self.Cube`)))))
  (`PrimitiveComponent.AddImpulseAtLocation` (`self.Cube`) (* _output_get_2 _output_get) _nearest_socket_location "None")
  (`GameplayStatics.SpawnEmitterAttached` "/Game/FXVarietyPack/Particles/P_ky_runePush.P_ky_runePush" _cube _nearest_socket_name (0.0 0.0 0.0) (`KismetMathLibrary.FindLookAtRotation` _nearest_socket_location CastPoint))
  (`GameplayStatics.SpawnSoundAttached` "/Game/Players/Audio/Wind_RunePush.Wind_RunePush" _cube "None" (0.0 0.0 0.0) (struct) "KeepRelativeOffset" false 1.0 1.0 0.0 null null))

(event `/Game/Players/Spells/BP_Spell_Interface.DeactivateSpell`)

(fn `AddForceFuncOld`
  (params (DeltaSeconds :type "Float (double-precision)"))
  (if (`self.Is Active`)
    (bind _output_get (set `self.Current Force` (+ (`self.Current Force`) (* 0.0 (`self.Delta Strength`))))) ; Increase force
    (bind _returnvalue (* (`self.ForceDirection`) (* _output_get DeltaSeconds)))
    (`PrimitiveComponent.AddForce` (`self.Cube`) _returnvalue "None" true)
    (`KismetSystemLibrary.PrintString` (`KismetStringLibrary.Conv_VectorToString` _returnvalue))))

(fn `GetNearestSocket`
  (params (ContactPoint :type "Vector Structure"))
  (returns (`Nearest Socket Name` :type Name) (`Nearest Socket Location` :type "Vector Structure") (`Nearest Socket Rotation` :type "Rotator Structure"))
  (locals (`Nearest Socket` :type Name))
  (bind _cube (`self.Cube`))
  (bind _nearest_socket (`local.Nearest Socket`))
  (bind _nearest_socket_2 (`local.Nearest Socket`))
  (bind _cube_2 (`self.Cube`))
  (for _array_element (`SceneComponent.GetAllSocketNames` _cube)
    (if (or (== _nearest_socket "None") (< (`KismetMathLibrary.VSize` (- (`SceneComponent.GetSocketLocation` _cube _array_element) ContactPoint)) (`KismetMathLibrary.VSize` (- (`SceneComponent.GetSocketLocation` _cube _nearest_socket) ContactPoint))))
      (set `local.Nearest Socket` _array_element)))
  (return _nearest_socket_2 (`SceneComponent.GetSocketLocation` _cube_2 _nearest_socket_2) (`SceneComponent.GetSocketRotation` _cube_2 _nearest_socket_2)))

(fn `UserConstructionScript`)