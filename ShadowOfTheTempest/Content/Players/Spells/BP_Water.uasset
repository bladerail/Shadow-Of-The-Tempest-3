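; BP_Water is a water actor, filed under player spells, that rises vertically when its Raise event is called.
; BeginPlay stores the starting Z, then Raise plays a timeline from the start, offsetting height by the curve value times RaiseAmount while keeping current X and Y.
; The construction script records an Origin 100 units below the actor, which nothing else in the shown graphs reads.
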(event `self.ReceiveBeginPlay`
  (bind (_returnvalue_x _returnvalue_y _returnvalue_z) (`KismetMathLibrary.BreakVector` (`self.K2_GetActorLocation`)))
  (set `self.StartHeight` _returnvalue_z))

(event `Raise`
  (bind (_returnvalue_x _returnvalue_y) (`KismetMathLibrary.BreakVector` (`self.K2_GetActorLocation`)))
  (bind (_direction _newtrack_0) (`Timeline|Timeline_0` :!via `PlayFromStart`)
    (:`Update`
      (`self.K2_SetActorLocation` (`KismetMathLibrary.MakeVector` _returnvalue_x _returnvalue_y (+ (`self.StartHeight`) (* (`self.RaiseAmount`) _newtrack_0)))))))

(fn `UserConstructionScript`
  (set `self.Origin` (- (`self.K2_GetActorLocation`) (0.0 0.0 100.0))))