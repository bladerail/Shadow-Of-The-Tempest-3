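; BP_StoneStatue is a player spell that conjures a BP_ShadowStatue in the world and removes it on deactivation.
; CastSpell calls ServerCast, which spawns the statue just ahead of the spell actor with matching rotation and scale, stores it, and plays a shadow conjuring sound.
; DeactivateSpell calls ServerDeactivate, which destroys the stored statue.
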(event `self.ReceiveBeginPlay`)

(event `/Game/Players/Spells/BP_Spell_Interface.CastSpell`
  (params (CastPoint :type "Vector Structure") (Strength :type "Float (single-precision)") (ContactPoint :type "Vector Structure"))
  (`self.Server Cast`))

(event `Server Cast`
  (bind (_returnvalue_location _returnvalue_rotation _returnvalue_scale) (`KismetMathLibrary.BreakTransform` (`self.GetTransform`)))
  (bind _returnvalue (`|SpawnActorFromClass` "/Game/Players/Spells/BP_ShadowStatue.BP_ShadowStatue_C" (`KismetMathLibrary.MakeTransform` (+ _returnvalue_location (* (`self.GetActorForwardVector`) 50.0)) _returnvalue_rotation _returnvalue_scale) "Undefined" "OverrideRootScale" null null))
  (set `self.CreatedStatue` _returnvalue)
  (`GameplayStatics.PlaySoundAtLocation` "/Game/Players/Audio/Shadow_ConjureShadow.Shadow_ConjureShadow" (`self.K2_GetActorLocation`) (struct) 1.0 1.0 0.0 null null null))

(event `/Game/Players/Spells/BP_Spell_Interface.DeactivateSpell`
  (`self.Server Deactivate`))

(event `Server Deactivate`
  (`self.K2_DestroyActor` (`self.CreatedStatue`)))

(fn `UserConstructionScript`)