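; BP_ProjBase is a spell projectile, apparently a base class, driven by a physics-simulated mesh and thruster that activate on spawn.
; Sphere overlaps send an attack message to any actor and also call BEATTACK on mybear.
; Hitting mybear or BP_DBG_Enemy, or reaching the fixed lifetime, spawns a shadow-ball hit effect at the mesh and destroys the actor.
; A scale-over-time timeline is present but never runs.
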(event `self.ReceiveBeginPlay`
  ;[1 1 1] BasicLogic
  (`PrimitiveComponent.SetSimulatePhysics` (`self.StaticMesh`) true)
  (`ActorComponent.SetActive` (`self.PhysicsThruster`) true false)
  (`ActorComponent.Activate` (`self.PhysicsThruster`) false)
  (`KismetSystemLibrary.Delay` 4.0)
  (`GameplayStatics.SpawnEmitterAtLocation` "/Game/FXVarietyPack/Particles/P_ky_shadowBallHit.P_ky_shadowBallHit" (`SceneComponent.K2_GetComponentLocation` (`self.StaticMesh`)) (struct) (1.0 1.0 1.0) false)
  (`self.K2_DestroyActor`))

(event `self.SphereCol.OnComponentBeginOverlap`
  (params (OverlappedComponent :type "PrimitiveComponent Object Reference") (OtherActor :type "Actor Object Reference") (OtherComp :type "PrimitiveComponent Object Reference") (OtherBodyIndex :type Integer) (bFromSweep :type Boolean) (SweepResult :type "HitResult Structure (by ref)"))
  (message `/Game/enemy/BP_enemy_be_attack.attack_from_projectile` OtherActor)
  (bind _asmybear (cast `/Game/enemy/bear/bear/mybear` OtherActor)
    (:`then`
      (`/Game/enemy/bear/bear/mybear.BEATTACK` _asmybear 0.0))
    (:`CastFailed`
      (cast `/Game/Players/HPBar/BP_DBG_Enemy` OtherActor)))
  (`GameplayStatics.SpawnEmitterAtLocation` "/Game/FXVarietyPack/Particles/P_ky_shadowBallHit.P_ky_shadowBallHit" (`SceneComponent.K2_GetComponentLocation` (`self.StaticMesh`)))
  (`self.K2_DestroyActor`))

(fn `UserConstructionScript`)