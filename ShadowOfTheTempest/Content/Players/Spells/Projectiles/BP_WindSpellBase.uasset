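; Base wind spell projectile that is propelled by physics and attacks bears it touches.
; On BeginPlay it enables mesh physics and a PhysicsThruster, then spawns an emitter and destroys itself after a ten-second lifetime.
; Sphere overlap with a mybear calls its BEATTACK, spawns a shockwave particle and destroys the projectile, ignoring other actors.
; A scale-over-time timeline is present but never runs.
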(event `self.ReceiveBeginPlay`
  ;[1 1 1] BasicLogic
  (`PrimitiveComponent.SetSimulatePhysics` (`self.StaticMesh`) true)
  (`ActorComponent.SetActive` (`self.PhysicsThruster`) true false)
  (`ActorComponent.Activate` (`self.PhysicsThruster`) false)
  (`KismetSystemLibrary.Delay` 10.0)
  (`GameplayStatics.SpawnEmitterAtLocation` null (`SceneComponent.K2_GetComponentLocation` (`self.StaticMesh`)) (struct) (1.0 1.0 1.0) false)
  (`self.K2_DestroyActor`))

(event `self.SphereCol.OnComponentBeginOverlap`
  (params (OverlappedComponent :type "PrimitiveComponent Object Reference") (OtherActor :type "Actor Object Reference") (OtherComp :type "PrimitiveComponent Object Reference") (OtherBodyIndex :type Integer) (bFromSweep :type Boolean) (SweepResult :type "HitResult Structure (by ref)"))
  (bind _asmybear (cast `/Game/enemy/bear/bear/mybear` OtherActor))
  (`/Game/enemy/bear/bear/mybear.BEATTACK` _asmybear)
  (`GameplayStatics.SpawnEmitterAtLocation` "/Game/FXVarietyPack/Particles/P_ky_spellShotShockwave.P_ky_spellShotShockwave" (`SceneComponent.K2_GetComponentLocation` (`self.StaticMesh`)))
  (`self.K2_DestroyActor`))

(fn `UserConstructionScript`)