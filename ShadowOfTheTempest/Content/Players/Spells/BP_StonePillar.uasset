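; Stone pillar spell target that conjures a shadow platform when cast on and can be toppled.
; CastSpell calls ServerCast, which plays shadow effects and spawns a BP_Platform beyond the pillar, opposite the cast point, scaled from mesh bounds like a cast shadow.
; DeactivateSpell destroys that platform through ServerDeactivate.
; BreakPillar runs a timeline that rolls and sinks the mesh, then plays a collapse sound.
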(event `self.ReceiveBeginPlay`)

(event `/Game/Players/Spells/BP_Spell_Interface.CastSpell`
  (params (CastPoint :type "Vector Structure") (Strength :type "Float (single-precision)") (ContactPoint :type "Vector Structure"))
  (`self.Server Cast` CastPoint))

(event `Server Cast`
  (params (`Cast Point` :type "Vector Structure"))
  (bind (_origin _boxextent) (`KismetSystemLibrary.GetComponentBounds` (`self.StaticMesh`)))
  (bind _returnvalue (`SceneComponent.K2_GetComponentLocation` (`self.StaticMesh`)))
  (bind _returnvalue_2 (- (`KismetMathLibrary.MakeVector` (.x _returnvalue) (.y _returnvalue)) (`KismetMathLibrary.MakeVector` (.x `Cast Point`) (.y `Cast Point`))))
  (`GameplayStatics.SpawnEmitterAttached` "/Game/FXVarietyPack/Particles/P_ky_shadowSpell.P_ky_shadowSpell" (`self.StaticMesh`) "None" (0.0 0.0 0.0) (struct) (0.5 0.5 1.0))
  (`GameplayStatics.PlaySoundAtLocation` "/Game/Players/Audio/Shadow_ConjurePlatform.Shadow_ConjurePlatform" _returnvalue (struct) 1.0 1.0 0.0 null null null)
  (bind _returnvalue_3 (`|SpawnActorFromClass` "/Game/Players/Spells/BP_Platform.BP_Platform_C" (`KismetMathLibrary.MakeTransform` (+ _returnvalue_2 (`self.K2_GetActorLocation`)) (`KismetMathLibrary.MakeRotFromX` _returnvalue_2) (`KismetMathLibrary.MakeVector` (/ (.z _boxextent) 35.0) (/ (.x _boxextent) 50.0) 1.0)) "Undefined" "OverrideRootScale" null null))
  (bind _output_get (set `self.CreatedPlatform` _returnvalue_3)))

(event `/Game/Players/Spells/BP_Spell_Interface.DeactivateSpell`
  (`self.Server Deactivate`))

(event `Server Deactivate`
  (`self.K2_DestroyActor` (`self.CreatedPlatform`)))

(event `EventBreak`
  (bind (_returnvalue_x _returnvalue_y) (`KismetMathLibrary.BreakVector` (`self.GetActorScale3D`)))
  (bind (_returnvalue_x_2 _returnvalue_y_2 _returnvalue_z) (`KismetMathLibrary.BreakVector` (`self.K2_GetActorLocation`)))
  (bind _staticmesh (`self.StaticMesh`))
  (bind (_direction _newtrack_0) (`Timeline|Timeline_0` :!via `PlayFromStart`)
    (:`Update`
      (`SceneComponent.K2_SetRelativeRotation` _staticmesh (`KismetMathLibrary.MakeRotator` (* _newtrack_0 90.0)) false false)
      (`SceneComponent.K2_SetWorldLocation` _staticmesh (`KismetMathLibrary.MakeVector` _returnvalue_x_2 _returnvalue_y_2 (+ _returnvalue_z (* _newtrack_0 -30.0 _returnvalue_y))) false false))
    (:`Finished`
      (`GameplayStatics.PlaySoundAtLocation` "/Game/Sounds/Pillar_collapse.Pillar_collapse" (`SceneComponent.K2_GetComponentLocation` (`self.StaticMesh`)) (struct) 1.0 1.0 0.0 null null null))))

(fn `BreakPillar`
  (`self.EventBreak`))

(fn `UserConstructionScript`)