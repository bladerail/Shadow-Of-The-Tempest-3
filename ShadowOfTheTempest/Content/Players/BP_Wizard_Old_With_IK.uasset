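; Player pawn for the old wizard, with camera-relative movement and look controls that support both VR headsets and controller-driven view.
; On BeginPlay the camera follows control rotation instead of locking to the HMD, and the tracking origin is set per headset, with PSVR using eye level plus a height offset and controller roll.
; Holding Q shifts the camera root sideways.
; Primary and secondary actions only print debug text, and the graphs contain no IK logic.
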(event `self.ReceiveBeginPlay`
  (bind _camera (`self.Camera`))
  (set `CameraComponent.bLockToHmd` false _camera)
  (set `CameraComponent.bUsePawnControlRotation` true _camera)
  (switch `name` (`HeadMountedDisplayFunctionLibrary.GetHMDDeviceName`)
    (:`Oculus HMD`
      (`HeadMountedDisplayFunctionLibrary.SetTrackingOrigin` "Floor" :!label _label))
    (:`SteamVR`
      (goto _label))
    (:`PSVR`
      (`HeadMountedDisplayFunctionLibrary.SetTrackingOrigin` "Eye")
      (`SceneComponent.K2_AddLocalOffset` (`self.CameraRoot`) (0.0 0.0 180.0) false false)
      (set `self.bUseControllerRotationRoll` true))))

(event `self.ReceiveTick`
  (params (DeltaSeconds :type "Float (single-precision)")))

(event `InputAxis|MoveForward`
  (params (AxisValue :type "Float (single-precision)"))
  (`self.AddMovementInput` (`SceneComponent.GetForwardVector` (`self.Camera`)) AxisValue))

(event `InputAxis|MoveRight`
  (params (AxisValue :type "Float (single-precision)"))
  (`self.AddMovementInput` (`SceneComponent.GetRightVector` (`self.Camera`)) AxisValue))

(event `InputAxis|Turn`
  (params (AxisValue :type "Float (single-precision)"))
  (`self.AddControllerYawInput` AxisValue))

(event `InputAxis|LookUp`
  (params (AxisValue :type "Float (single-precision)"))
  (`self.AddControllerPitchInput` AxisValue))

(event `InputAxis|TurnRate`
  (params (AxisValue :type "Float (single-precision)"))
  (`self.AddControllerYawInput` (* AxisValue (`self.BaseTurnRate`) (`GameplayStatics.GetWorldDeltaSeconds`))))

(event `InputAxis|LookUpRate`
  (params (AxisValue :type "Float (single-precision)"))
  (`self.AddControllerPitchInput` (* AxisValue (`self.BaseLookUpRate`) (`GameplayStatics.GetWorldDeltaSeconds`))))

(event `InputAction|PrimaryAction`
  (params (Key :type "Key Structure"))
  (:`Pressed`
    (`KismetSystemLibrary.PrintString` "Primary Action triggered")))

(event `InputAction|SecondaryAction`
  (params (Key :type "Key Structure"))
  (:`Pressed`
    (`KismetSystemLibrary.PrintString` "Secondary Action triggered")))

(event `Key|Q`
  (params (Key :type "Key Structure"))
  (:`Pressed`
    (`SceneComponent.K2_SetRelativeLocation` (`self.CameraRoot`) (0.0 -200.0 0.0) false false))
  (:`Released`
    (`SceneComponent.K2_SetRelativeLocation` (`self.CameraRoot`) (0.0 0.0 0.0) false false)))

(fn `UserConstructionScript`)