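; BP_SimpleProjectile is the player's spell projectile, spawning a color-tinted shockwave and shot sound on BeginPlay.
; It deactivates and destroys itself after Lifetime, or on capsule overlap, flagging whether it hit a BP_GenericEnemy and briefly delaying destruction if so.
; A Tick countdown lets EndPlay detect early destruction and play either full impact effects or half-scale miss effects with matching sound.
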(event `self.ReceiveBeginPlay`
  (bind _defaultsceneroot (`self.DefaultSceneRoot`))
  (bind _returnvalue (`SceneComponent.K2_GetComponentLocation` _defaultsceneroot))
  ;[1 1 1] spawn shot shockwave
  (set `self.Duration` (`self.Lifetime`))
  (bind _returnvalue_2 (`GameplayStatics.SpawnEmitterAtLocation` "/Game/FXVarietyPack/Particles/P_ky_spellShotShockwave.P_ky_spellShotShockwave" _returnvalue (`SceneComponent.K2_GetComponentRotation` _defaultsceneroot)))
  (`GameplayStatics.PlaySoundAtLocation` "/Game/Players/Audio/Player_ShootSpell.Player_ShootSpell" _returnvalue (struct) 1.0 1.0 0.0 null null null)
  (`ParticleSystemComponent.SetVectorParameter` _returnvalue_2 "color" (`KismetMathLibrary.Conv_LinearColorToVector` (`self.color`)))
  ;[1 1 1] Destroy projectile after lifetime is over
  (`KismetSystemLibrary.Delay` (`self.Lifetime`))
  (`ActorComponent.SetActive` (`self.SpellProjectile`) false false)
  (`KismetSystemLibrary.Delay` 0.5)
  (`self.K2_DestroyActor`))

(event `self.ReceiveTick`
  (params (DeltaSeconds :type "Float (single-precision)"))
  ;[1 1 1] Duration decrement for control
  (set `self.duration` (- (`self.duration`) DeltaSeconds)))

(event `self.Capsule.OnComponentBeginOverlap`
  (params (OverlappedComponent :type "PrimitiveComponent Object Reference") (OtherActor :type "Actor Object Reference") (OtherComp :type "PrimitiveComponent Object Reference") (OtherBodyIndex :type Integer) (bFromSweep :type Boolean) (SweepResult :type "HitResult Structure (by ref)"))
  ;[1 1 1] Destroy actor when it hits another actor
  (`KismetSystemLibrary.PrintString` (`KismetSystemLibrary.GetDisplayName` OtherActor))
  (if (`KismetSystemLibrary.IsValid` OtherActor)
    (cast `/Game/Enemies/BP_GenericEnemy` OtherActor
      (:`then`
        (set `self.HitEnemy` true)
        (`KismetSystemLibrary.Delay` 0.2)
        (`self.K2_DestroyActor`))
      (:`CastFailed`
        (set `self.HitEnemy` false)
        (`self.K2_DestroyActor`)))))

(event `self.ReceiveEndPlay`
  (params (EndPlayReason :type "EEndPlayReason Enum" :default "Destroyed"))
  (bind _spellhitfx (`self.SpellHitFx`))
  (bind _returnvalue (`SceneComponent.K2_GetComponentLocation` (`self.SpellProjectile`)))
  ;[1 1 1] Spawn FX and sound iff the projectile hit
  (if (> (`self.Duration`) 0.0)
    (if (`self.HitEnemy`)
      (`GameplayStatics.SpawnEmitterAtLocation` _spellhitfx _returnvalue)
      (`GameplayStatics.PlaySoundAtLocation` "/Game/Players/Audio/Player_SpellImpact.Player_SpellImpact" _returnvalue (struct) 1.0 1.0 0.0 null null null)
      (else
        (`GameplayStatics.SpawnEmitterAtLocation` _spellhitfx _returnvalue (struct) (0.5 0.5 0.5))
        (`GameplayStatics.PlaySoundAtLocation` "/Game/Players/Audio/Player_SpellMiss.Player_SpellMiss" _returnvalue (struct) 1.0 1.0 0.0 null null null)))))

(fn `MissHitbox`
  (set `self.HitEnemy` false)
  (`self.K2_DestroyActor`))

(fn `UserConstructionScript`)