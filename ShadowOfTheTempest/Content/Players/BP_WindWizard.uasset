(event `Client Deactivate Portcullis`
  (params (Portcullis :type "/Game/Props/BP_Doorway Object Reference") (`Particle Effect` :type "ParticleSystemComponent Object Reference"))
  ;[1 1 1] Wind Wizard Deactivate Portcullis Spell
  (`self.Server Deactivate Portcullis` Portcullis `Particle Effect`))

(event `Wind Deactivate Portcullis`
  (params (Portcullis :type "/Game/Props/BP_Doorway Object Reference") (`Particle Effect` :type "ParticleSystemComponent Object Reference"))
  ;[1 1 1] Wind Wizard Deactivate Portcullis Spell
  (bind _asnew_game_instance (cast `/Game/Networking/NewGameInstance` (`GameplayStatics.GetGameInstance`)))
  (if (`/Game/Networking/NewGameInstance.IsServer` _asnew_game_instance)
    (`self.Server Deactivate Portcullis` Portcullis `Particle Effect`)
    (else
      (`self.Client Deactivate Portcullis` Portcullis `Particle Effect`))))

(event `Server Deactivate Portcullis`
  (params (Portcullis :type "/Game/Props/BP_Doorway Object Reference") (`Particle Effect` :type "ParticleSystemComponent Object Reference"))
  ;[1 1 1] Wind Wizard Deactivate Portcullis Spell
  (set `/Game/Props/BP_Doorway.CurrentSpeed` (`/Game/Props/BP_Doorway.OriginalSpeed` Portcullis) Portcullis)
  (`ActorComponent.SetActive` `Particle Effect` false false))

(event `self.ReceiveBeginPlay`
  (`parent.ReceiveBeginPlay`)
  (`KismetSystemLibrary.PrintString` "Spawn wind"))

(event `Client Cast Portcullis`
  (params (Strength :type "Float (double-precision)") (Doorway :type "/Game/Props/BP_Doorway Object Reference"))
  ;[1 1 1] Wind Wizard Cast Portcullis Spell
  (`self.Server Cast Portcullis` Strength Doorway))

(event `Wind Cast Portcullis`
  (params (Strength :type "Float (double-precision)") (Doorway :type "/Game/Props/BP_Doorway Object Reference"))
  ;[1 1 1] Wind Wizard Cast Portcullis Spell
  (bind _asnew_game_instance (cast `/Game/Networking/NewGameInstance` (`GameplayStatics.GetGameInstance`)))
  (if (`/Game/Networking/NewGameInstance.IsServer` _asnew_game_instance)
    (`self.Server Cast Portcullis` Strength Doorway)
    (else
      (`self.Client Cast Portcullis` Strength Doorway))))

(event `Server Cast Portcullis`
  (params (Strength :type "Float (double-precision)") (Doorway :type "/Game/Props/BP_Doorway Object Reference"))
  ;[1 1 1] Wind Wizard Cast Portcullis Spell
  (if (`|EnumEquality` (`/Game/Props/BP_Doorway.CurrentState` Doorway) "NewEnumerator0")
    (set `/Game/Props/BP_Doorway.CurrentSpeed` (- (`/Game/Props/BP_Doorway.OriginalSpeed` Doorway) Strength) Doorway)))

(event `Server Cast Spell`
  (params (Strength :type "Float (double-precision)"))
  (`self.CastSpell` Strength))

(event `InputAction|Fire`
  (params (Key :type "Key Structure"))
  (bind _leftcontroller (`self.LeftController`))
  (bind _leftcontroller_2 (`self.LeftController`))
  (bind _returnvalue (`SceneComponent.K2_GetComponentRotation` (`self.Camera`)))
  (bind _returnvalue_2 (`SceneComponent.K2_GetComponentRotation` (`self.Camera`)))
  (bind _returnvalue_3 (+ (`SceneComponent.K2_GetComponentLocation` (`self.ProjectileSpawn`)) (`KismetMathLibrary.GreaterGreater_VectorRotator` (`self.ShootOffset`) _returnvalue)))
  (bind _returnvalue_4 (+ (`SceneComponent.K2_GetComponentLocation` (`self.ProjectileSpawn`)) (`KismetMathLibrary.GreaterGreater_VectorRotator` (`self.ShootOffset`) _returnvalue_2)))
  (:`Pressed`
    (bind _asnew_game_instance (cast `/Game/Networking/NewGameInstance` (`GameplayStatics.GetGameInstance`)))
    (if (`/Game/Networking/NewGameInstance.IsServer` _asnew_game_instance)
      (if (`/Game/VirtualRealityBP/Blueprints/BP_MotionController.Laser` _leftcontroller_2)
        (`self.Server Fire Wind` (`KismetMathLibrary.MakeTransform` _returnvalue_4 (`SceneComponent.K2_GetComponentRotation` (`/Game/VirtualRealityBP/Blueprints/BP_MotionController.LaserSystem` _leftcontroller_2))))
        (else
          (`self.Server Fire Wind` (`KismetMathLibrary.MakeTransform` _returnvalue_4 _returnvalue_2))))
      (elif (`/Game/VirtualRealityBP/Blueprints/BP_MotionController.Laser` _leftcontroller)
        (`self.Client Fire Wind` (`KismetMathLibrary.MakeTransform` _returnvalue_3 (`SceneComponent.K2_GetComponentRotation` (`/Game/VirtualRealityBP/Blueprints/BP_MotionController.LaserSystem` _leftcontroller))))
        (else
          (`self.Client Fire Wind` (`KismetMathLibrary.MakeTransform` _returnvalue_3 _returnvalue)))))))

(event `InputAction|Spell1`
  (params (Key :type "Key Structure"))
  (bind _strength (`self.Strength`))
  (:`Pressed`
    (bind _asnew_game_instance (cast `/Game/Networking/NewGameInstance` (`GameplayStatics.GetGameInstance`)))
    (if (`/Game/Networking/NewGameInstance.IsServer` _asnew_game_instance)
      (`self.Server Cast Spell` _strength)
      (else
        (`self.Client Cast Spell` _strength)))))

(event `Client Cast Spell`
  (params (Strength :type "Float (double-precision)"))
  (`self.Server Cast Spell` Strength))

(event `InputAction|Spell2`
  (params (Key :type "Key Structure"))
  (:`Pressed`
    (bind _asnew_game_instance (cast `/Game/Networking/NewGameInstance` (`GameplayStatics.GetGameInstance`)))
    (if (`/Game/Networking/NewGameInstance.IsServer` _asnew_game_instance)
      (`self.Server Cast Spell` 0.0)
      (else
        (`self.Client Cast Spell` (* (`self.Strength`) -1.0))))))

(event `self.SetNewActiveSpell`
  (params (NewSpellActor :type "Actor Object Reference"))
  (bind _activespellonmap (`self.ActiveSpellOnMap`))
  (if (== _activespellonmap null)
    (cast `/Game/Players/Spells/BP_RuneBox` NewSpellActor ; If new == RuneBox, set to nil
      (:`then`
        (set `self.ActiveSpellOnMap` null :!label _label))
      (:`CastFailed`
        (set `self.ActiveSpellOnMap` NewSpellActor :!label _label_2)))
    (elif (== NewSpellActor null)
      (goto _label)
      (elif (== NewSpellActor _activespellonmap)
        (bind _asbp_spell_interface (cast `/Game/Players/Spells/BP_Spell_Interface` _activespellonmap) ; If old == new, deactivate old and set nil
          (:`then`
            (`/Game/Players/Spells/BP_Spell_Interface.DeactivateSpell` _asbp_spell_interface)
            (goto _label))
          (:`CastFailed`
            (goto _label)))
        (else
          (bind _asbp_spell_interface_2 (cast `/Game/Players/Spells/BP_Spell_Interface` _activespellonmap) ; If old != new, deactivate old, cast new, set new
            (:`then`
              (`/Game/Players/Spells/BP_Spell_Interface.DeactivateSpell` _asbp_spell_interface_2)
              (goto _label_2))
            (:`CastFailed`
              (if (<= (`KismetArrayLibrary.Array_Length` (`PrimitiveComponent.GetOverlappingActors` (`self.CapsuleComponent`) "/Game/Players/Spells/BP_Water.BP_Water_C")) 0)
                (`self.StopLevitateSpell`)
                (goto _label_2)))))))))

(event `Server Fire Wind`
  (params (SpawnTransform :type "Transform Structure"))
  (`self.PlayRandomAttackAnimation`)
  (`|SpawnActorFromClass` "/Game/Players/BP_WindProjectile.BP_WindProjectile_C" SpawnTransform "Undefined" "OverrideRootScale" null null))

(event `Client Fire Wind`
  (params (SpawnTransform :type "Transform Structure"))
  (`self.Server Fire Wind` SpawnTransform))

(event `self.ExtinguishTorchSphere.OnComponentBeginOverlap`
  (params (OverlappedComponent :type "PrimitiveComponent Object Reference") (OtherActor :type "Actor Object Reference") (OtherComp :type "PrimitiveComponent Object Reference") (OtherBodyIndex :type Integer) (bFromSweep :type Boolean) (SweepResult :type "HitResult Structure (by ref)"))
  (if (`self.IsLevitating`)
    (bind _asbp_torch (cast `/Game/MedievalDungeon/Blueprints/BP_Torch` OtherActor))
    (`/Game/MedievalDungeon/Blueprints/BP_Torch.TurnOffTorch` _asbp_torch)))

(event `self.ExtinguishTorchSphere.OnComponentEndOverlap`
  (params (OverlappedComponent :type "PrimitiveComponent Object Reference") (OtherActor :type "Actor Object Reference") (OtherComp :type "PrimitiveComponent Object Reference") (OtherBodyIndex :type Integer))
  (bind _asbp_torch (cast `/Game/MedievalDungeon/Blueprints/BP_Torch` OtherActor))
  (`/Game/MedievalDungeon/Blueprints/BP_Torch.TurnOnTorch` _asbp_torch))

(event `self.CapsuleComponent.OnComponentBeginOverlap`
  (params (OverlappedComponent :type "PrimitiveComponent Object Reference") (OtherActor :type "Actor Object Reference") (OtherComp :type "PrimitiveComponent Object Reference") (OtherBodyIndex :type Integer) (bFromSweep :type Boolean) (SweepResult :type "HitResult Structure (by ref)"))
  ;[1 1 1] Raise and lower Camera artificially to give the effect of actual levitation
  (cast `/Game/Players/Spells/BP_Water` OtherActor)
  (if (`self.IsLevitating`)
    (`SceneComponent.K2_SetRelativeLocation` (`self.Camera`) (5.0 0.0 50.0) false false)))

(event `self.CapsuleComponent.OnComponentEndOverlap`
  (params (OverlappedComponent :type "PrimitiveComponent Object Reference") (OtherActor :type "Actor Object Reference") (OtherComp :type "PrimitiveComponent Object Reference") (OtherBodyIndex :type Integer))
  ;[1 1 1] Raise and lower Camera artificially to give the effect of actual levitation
  (cast `/Game/Players/Spells/BP_Water` OtherActor)
  (if (`self.IsLevitating`)
    (`SceneComponent.K2_SetRelativeLocation` (`self.Camera`) (5.0 0.0 0.0) false false)))

(event `Client Set Health`
  (params (Damage :type Integer))
  (set `self.Health` (- (`self.Health`) Damage)))

(event `self.ReceiveDamage`
  (params (Damage :type Integer))
  (bind _damageoverlay (`self.DamageOverlay`))
  (bind _returnvalue (`WidgetComponent.GetUserWidgetObject` _damageoverlay))
  (bind _asnew_game_instance (cast `/Game/Networking/NewGameInstance` (`GameplayStatics.GetGameInstance`)))
  (if (not (`/Game/Networking/NewGameInstance.IsServer` _asnew_game_instance))
    (`self.Client Set Health` Damage)
    (`GameplayStatics.PlaySoundAtLocation` "/Game/Players/Audio/Player_BodyHit.Player_BodyHit" (`self.K2_GetActorLocation`) (struct) 1.0 1.0 0.0 null null null)
    (`KismetSystemLibrary.PrintString` "OH!")
    (if (< (`KismetMathLibrary.Conv_IntToDouble` (`self.Health`)) 1.0)
      (`KismetSystemLibrary.PrintString` "you die!"))
    (bind _returnvalue_2 (`|CreateWidget` "/Game/enemy/BP_DamageWidget.BP_DamageWidget_C"))
    (`WidgetComponent.SetWidget` _damageoverlay _returnvalue_2)
    (`UserWidget.AddToViewport` _returnvalue 0)
    (`KismetSystemLibrary.Delay` 0.2)
    (`Widget.RemoveFromParent` _returnvalue)))

(fn `CastLevitateSpell`
  (params (Height :type "Float (double-precision)"))
  (locals (`Z Offset` :type "Float (double-precision)" :default 50.0))
  (bind _returnvalue (<= (`KismetArrayLibrary.Array_Length` (`PrimitiveComponent.GetOverlappingActors` (`self.CapsuleComponent`) "/Game/Players/Spells/BP_Water.BP_Water_C")) 0))
  (if (`self.IsLevitating`)
    (if _returnvalue
      (`self.StopLevitateSpell`)
      (`self.SetNewActiveSpell` null)
      (`KismetSystemLibrary.PrintString` (`KismetStringLibrary.Conv_BoolToString` (`self.IsLevitating`)) :!label _label)
      (set `self.CanCastSpell` true)
      (else
        (`KismetSystemLibrary.PrintString` "Hello")
        (set `self.CanCastSpell` false)))
    (else
      (`PrimitiveComponent.SetCollisionObjectType` (`self.CapsuleComponent`) "ECC_GameTraceChannel3")
      (set `self.IsLevitating` true)
      (if (not _returnvalue)
        ;[1 1 1] If wizard already overlapped with water and is just now casting levitate, raise the camera
        (`SceneComponent.K2_SetRelativeLocation` (`self.Camera`) (5.0 0.0 50.0) false false))
      (`self.SetNewActiveSpell` self)
      (`AudioComponent.Play` (`self.AttachedSound`) 0.0)
      (`ActorComponent.SetActive` (`self.ParticleSystem`) true false)
      (`self.SwitchOffTorches`)
      (goto _label))))

(fn `CastPortcullisSpell`
  (params (`Target Portcullis` :type "/Game/Props/BP_Doorway Object Reference") (Strength :type "Float (double-precision)"))
  (`/Game/Props/BP_Doorway.CastSpell` `Target Portcullis` (0.0 0.0 0.0) Strength (0.0 0.0 0.0))
  (`self.SetNewActiveSpell` `Target Portcullis`))

(fn `CastSpell`
  (params (Strength :type "Float (double-precision)"))
  (bind _returnvalue (`self.K2_GetActorLocation`))
  (bind (_actor _component _location) (`self.GetTarget`))
  (bind _asbp_spell_interface (cast `/Game/Players/Spells/BP_Spell_Interface` _actor)
    (:`then`
      (bind _asbp_rune_box (cast `/Game/Players/Spells/BP_RuneBox` (`KismetSystemLibrary.Conv_InterfaceToObject` _asbp_spell_interface))
        (:`then`
          (`/Game/Players/Spells/BP_Spell_Interface.CastSpell` _asbp_rune_box _returnvalue Strength _location)
          (`self.SetNewActiveSpell` null))
        (:`CastFailed`
          (`self.SetNewActiveSpell` _actor)
          (if (not (== (`self.ActiveSpellOnMap`) null))
            (`/Game/Players/Spells/BP_Spell_Interface.CastSpell` _asbp_spell_interface _returnvalue Strength _location)))))
    (:`CastFailed`
      (`self.CastLevitateSpell` 0.0))))

(fn `StopLevitateSpell`
  (set `self.IsLevitating` false)
  (`AudioComponent.Stop` (`self.AttachedSound`))
  (`ActorComponent.SetActive` (`self.ParticleSystem`) false false)
  (`PrimitiveComponent.SetCollisionObjectType` (`self.CapsuleComponent`) "ECC_Pawn")
  (`self.SwitchOnTorches`))

(fn `SwitchOffTorches`
  (for _array_element (`PrimitiveComponent.GetOverlappingActors` (`self.ExtinguishTorchSphere`) null)
    (bind _asbp_torch (cast `/Game/MedievalDungeon/Blueprints/BP_Torch` _array_element))
    (`/Game/MedievalDungeon/Blueprints/BP_Torch.TurnOffTorch` _asbp_torch)))

(fn `SwitchOnTorches`
  (for _array_element (`PrimitiveComponent.GetOverlappingActors` (`self.ExtinguishTorchSphere`) null)
    (bind _asbp_torch (cast `/Game/MedievalDungeon/Blueprints/BP_Torch` _array_element))
    (`/Game/MedievalDungeon/Blueprints/BP_Torch.TurnOnTorch` _asbp_torch)))

(fn `UserConstructionScript`
  (`ParticleSystemComponent.SetColorParameter` (`self.ParticleSystem`) "color" (`self.Color`)))