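; BP_HPRunes_UV is a health indicator actor that shows HP as eight text-render runes.
; UpdateHP, run by HPChangeEvent and with placeholder values at BeginPlay, computes the HP fraction and checks each rune against a rising threshold.
; ChangeRune swaps between two UV text materials by that threshold; its rune-scaling nodes are disconnected.
; UpdateLocation snaps the root to AttachTarget, but nothing in this Blueprint calls it.
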(event `self.ReceiveBeginPlay`
  (`self.UpdateHP` 80.0 100.0))

(event `self.ReceiveTick`
  (params (DeltaSeconds :type "Float (single-precision)")))

(event `HPChangeEvent`
  (params (HP :type "Float (double-precision)") (HPUB :type "Float (double-precision)"))
  (`self.UpdateHP` HP HPUB))

(fn `ChangeRune`
  (params (TextRender :type "TextRenderComponent Object Reference") (HPLevel :type "Float (double-precision)"))
  (if (>= (`self.HPPct`) HPLevel)
    (`TextRenderComponent.SetTextMaterial` TextRender "/Game/UVLight/Materials/M_UVText.M_UVText")
    (else
      (`TextRenderComponent.SetTextMaterial` TextRender "/Game/UVLight/Materials/M_UVText_2.M_UVText_2")))
  (return))

(fn `UpdateHP`
  (params (HP :type "Float (double-precision)") (HPUB :type "Float (double-precision)"))
  (set `self.HPPct` (/ HP HPUB))
  (`self.ChangeRune` (`self.Rune1`) 0.125)
  (`self.ChangeRune` (`self.Rune3`) 0.25)
  (`self.ChangeRune` (`self.Rune4`) 0.375)
  (`self.ChangeRune` (`self.Rune5`) 0.5)
  (`self.ChangeRune` (`self.Rune6`) 0.625)
  (`self.ChangeRune` (`self.Rune8`) 0.75)
  (`self.ChangeRune` (`self.Rune9`) 0.875)
  (`self.ChangeRune` (`self.Rune10`) 0.99))

(fn `UpdateLocation`
  (bind _attachtarget (`self.AttachTarget`))
  (if (not (== _attachtarget null))
    (`SceneComponent.K2_SetWorldLocation` (`self.DefaultSceneRoot`) (`self.K2_GetActorLocation` _attachtarget) false false)))

(fn `UserConstructionScript`)