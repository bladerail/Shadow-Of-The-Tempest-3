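; BP_DBG_Enemy is an enemy actor, apparently for debugging, with a world-space health bar that faces the player's VR camera.
; HitbyGate subtracts damage from HP, while HitBySpell is a stub that returns false.
; UpdateHP sets the widget's progress bar against a fixed maximum and notifies HPRune if valid; HitbyGate also notifies the rune directly.
; Tick rotates the widget toward the camera each frame.
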(event `self.ReceiveBeginPlay`
  (`self.UpdateHP` (`self.HP`) 100.0))

(event `self.ReceiveTick`
  (params (DeltaSeconds :type "Float (single-precision)"))
  (`self.UpdateBarDirection`))

(event `/Game/Players/Combat/BPI_Combat.HitByGate`
  (params (Damage :type "Float (single-precision)"))
  (bind _returnvalue (- (`self.HP`) Damage))
  (`self.UpdateHP` _returnvalue 100.0)
  (bind _output_get (set `self.HP` _returnvalue))
  (`/Game/Players/HPBar/BP_HPRunes_UV.HPChangeEvent` (`self.HPRune`) _output_get 100.0))

(fn `HitBySpell`
  (params (Damage :type "Float (double-precision)"))
  (returns (qqq :type Boolean))
  (return false))

(fn `UpdateBarDirection`
  (bind _location (`/Game/Utility/LayoutVRUtilityFunctions.Get Player VR Camera Properties`))
  (`SceneComponent.K2_SetWorldRotation` (`self.Widget`) (`KismetMathLibrary.FindLookAtRotation` (`SceneComponent.K2_GetComponentLocation` (`self.Widget`)) _location) false false))

(fn `UpdateHP`
  (params (HP :type "Float (double-precision)") (HPUB :type "Float (double-precision)"))
  (bind _hprune (`self.HPRune`))
  (bind _aswidget_enemy_health_bar (cast `/Game/Players/HPBar/Widget_EnemyHealthBar` (`WidgetComponent.GetUserWidgetObject` (`self.Widget`))))
  (`ProgressBar.SetPercent` (`/Game/Players/HPBar/Widget_EnemyHealthBar.ProgressBar_88` _aswidget_enemy_health_bar) (/ HP HPUB))
  (if (`KismetSystemLibrary.IsValid` _hprune)
    (`/Game/Players/HPBar/BP_HPRunes_UV.HPChangeEvent` _hprune HP HPUB)))

(fn `UserConstructionScript`)