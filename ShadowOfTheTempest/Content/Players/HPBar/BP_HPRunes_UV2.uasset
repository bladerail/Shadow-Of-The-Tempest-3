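; Floating HP bar actor that follows an attach target and shows health as eight rune text actors.
; BeginPlay spawns blue runes, applies an initial 80% HP and spreads their scene anchors by a radius multiplier.
; HP updates replace runes above the current fraction with alternate-class "X" runes, never restoring blue ones.
; Tick follows the target, snaps runes to their anchors and randomly jitters anchor height within bounds.
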(event `self.ReceiveBeginPlay`
  (`self.CreateAllRunes`)
  (`self.UpdateHP` 80.0 100.0)
  (`self.ScaleThisActor` 3.0))

(event `self.ReceiveTick`
  (params (DeltaSeconds :type "Float (single-precision)"))
  (`self.UpdateLocation`)
  (`self.UpdateAllRunes`))

(event `HPChangeEvent`
  (params (HP :type "Float (double-precision)") (HPUB :type "Float (double-precision)"))
  (`self.UpdateHP` HP HPUB))

(fn `AttachHPBarTo`
  (params (AttachTarget :type "Actor Object Reference"))
  (set `self.AttachTarget` AttachTarget))

(fn `ChangeRune`
  (params (Rune :type "Actor Object Reference") (HPLevel :type "Float (double-precision)"))
  (returns (NewRune :type "Actor Object Reference"))
  (if (>= (`self.HPPct`) HPLevel)
    (return Rune)
    (else
      (`self.K2_DestroyActor` Rune)
      (bind _textref (`self.CreateRune` false "X"))
      (return _textref))))

(fn `CreateAllRunes`
  (bind _textref (`self.CreateRune` true "O"))
  (set `self.RuneRef1` _textref)
  (bind _textref_2 (`self.CreateRune` true "X"))
  (set `self.RuneRef2` _textref_2)
  (bind _textref_3 (`self.CreateRune` true "Y"))
  (set `self.RuneRef3` _textref_3)
  (bind _textref_4 (`self.CreateRune` true "Z"))
  (set `self.RuneRef4` _textref_4)
  (bind _textref_5 (`self.CreateRune` true "E"))
  (set `self.RuneRef5` _textref_5)
  (bind _textref_6 (`self.CreateRune` true "Q"))
  (set `self.RuneRef6` _textref_6)
  (bind _textref_7 (`self.CreateRune` true "S"))
  (set `self.RuneRef7` _textref_7)
  (bind _textref_8 (`self.CreateRune` true "H"))
  (set `self.RuneRef8` _textref_8))

(fn `CreateRune`
  (params (ColorIsBlue :type Boolean) (Text :type Text))
  (returns (TextRef :type "Actor Object Reference"))
  (bind _returnvalue (`KismetMathLibrary.MakeTransform` (0.0 0.0 0.0)))
  (if ColorIsBlue
    (bind _returnvalue_2 (`|SpawnActorFromClass` "/Game/Players/HPBar/BP_UVHPText.BP_UVHPText_C" _returnvalue "Undefined" "OverrideRootScale" null null))
    (`TextRenderComponent.K2_SetText` (`/Game/Players/HPBar/BP_UVHPText.TextRender` _returnvalue_2) Text)
    (return _returnvalue_2)
    (else
      (bind _returnvalue_3 (`|SpawnActorFromClass` "/Game/Players/HPBar/BP_UVHPText_2.BP_UVHPText_2_C" _returnvalue "Undefined" "OverrideRootScale" null null))
      (`TextRenderComponent.K2_SetText` (`/Game/Players/HPBar/BP_UVHPText_2.TextRender` _returnvalue_3) Text)
      (return _returnvalue_3))))

(fn `RuneRandomFloat`
  (params (Target :type "ActorComponent Object Reference"))
  (bind _asscene_component (cast `SceneComponent` Target))
  (bind (_relativelocation_x _relativelocation_y _relativelocation_z) (`KismetMathLibrary.BreakVector` (`SceneComponent.RelativeLocation` _asscene_component)))
  (bind _returnvalue (+ _relativelocation_z (`KismetMathLibrary.RandomFloatInRange` -0.2 0.2)))
  (if (and (>= _returnvalue -5.0) (<= _returnvalue 5.0))
    (`SceneComponent.K2_SetRelativeLocation` _asscene_component (`KismetMathLibrary.MakeVector` _relativelocation_x _relativelocation_y _returnvalue) false false)))

(fn `ScaleThisActor`
  (params (Radius :type "Float (double-precision)") (TextSize :type "Float (double-precision)"))
  (for _array_element (`|MakeArray` (`self.Scene1`) (`self.Scene2`) (`self.Scene3`) (`self.Scene4`) (`self.Scene5`) (`self.Scene6`) (`self.Scene7`) (`self.Scene8`))
    (`SceneComponent.K2_SetRelativeLocation` _array_element (* (`SceneComponent.RelativeLocation` _array_element) Radius) false false)))

(fn `SetupHPBar`
  (params (R :type "Float (double-precision)") (Actor :type "Actor Object Reference"))
  (set `self.Radius` R)
  (set `self.AttachTarget` Actor))

(fn `UpdateAllRunes`
  (for (_array_element _array_index) (`|MakeArray` (`self.RuneRef1`) (`self.RuneRef2`) (`self.RuneRef3`) (`self.RuneRef4`) (`self.RuneRef5`) (`self.RuneRef6`) (`self.RuneRef7`) (`self.RuneRef8`))
    (bind _output (`|GetArrayItem` (`|MakeArray` (`self.Scene1`) (`self.Scene2`) (`self.Scene3`) (`self.Scene4`) (`self.Scene5`) (`self.Scene6`) (`self.Scene7`) (`self.Scene8`)) _array_index))
    (`self.UpdateRune` _array_element _output)
    (`self.RuneRandomFloat` _output)))

(fn `UpdateHP`
  (params (HP :type "Float (double-precision)") (HPUB :type "Float (double-precision)"))
  (set `self.HPPct` (/ HP HPUB))
  (bind _newrune (`self.ChangeRune` (`self.RuneRef1`) 0.125))
  (set `self.RuneRef1` _newrune)
  (bind _newrune_2 (`self.ChangeRune` (`self.RuneRef2`) 0.25))
  (set `self.RuneRef2` _newrune_2)
  (bind _newrune_3 (`self.ChangeRune` (`self.RuneRef3`) 0.375))
  (set `self.RuneRef3` _newrune_3)
  (bind _newrune_4 (`self.ChangeRune` (`self.RuneRef4`) 0.5))
  (set `self.RuneRef4` _newrune_4)
  (bind _newrune_5 (`self.ChangeRune` (`self.RuneRef5`) 0.625))
  (set `self.RuneRef5` _newrune_5)
  (bind _newrune_6 (`self.ChangeRune` (`self.RuneRef6`) 0.75))
  (set `self.RuneRef6` _newrune_6)
  (bind _newrune_7 (`self.ChangeRune` (`self.RuneRef7`) 0.875))
  (set `self.RuneRef7` _newrune_7)
  (bind _newrune_8 (`self.ChangeRune` (`self.RuneRef8`) 0.99))
  (set `self.RuneRef8` _newrune_8))

(fn `UpdateLocation`
  (bind _attachtarget (`self.AttachTarget`))
  (if (not (== _attachtarget null))
    (`SceneComponent.K2_SetWorldLocation` (`self.DefaultSceneRoot`) (`self.K2_GetActorLocation` _attachtarget) false false)))

(fn `UpdateRune`
  (params (RuneTextActor :type "Actor Object Reference") (AttachScene :type "ActorComponent Object Reference"))
  (bind _asscene_component (cast `SceneComponent` AttachScene))
  (cast `/Game/Players/HPBar/BP_UVHPText` RuneTextActor
    (:`then`
      (bind _returnvalue (`SceneComponent.K2_GetComponentLocation` _asscene_component))
      (bind _returnvalue_2 (`SceneComponent.K2_GetComponentRotation` _asscene_component))
      (`self.K2_SetActorLocationAndRotation` RuneTextActor _returnvalue _returnvalue_2 false false))
    (:`CastFailed`
      (cast `/Game/Players/HPBar/BP_UVHPText_2` RuneTextActor)
      (`self.K2_SetActorLocationAndRotation` RuneTextActor _returnvalue _returnvalue_2 false false))))

(fn `UserConstructionScript`)