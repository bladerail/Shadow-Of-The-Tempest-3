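; BP_Wisp is a player marker actor that glides toward a commanded world position.
; The Move event stores the target, and Tick steps toward it at MoveSpeed without sweeping, clamping each step to the remaining distance to avoid overshoot.
; The construction script picks the player 1 or player 2 marker particle template from the IsPlayer1 flag.
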(event `self.ReceiveTick`
  (params (DeltaSeconds :type "Float (single-precision)"))
  (bind _returnvalue (- (`self.NextPos`) (`self.K2_GetActorLocation`)))
  (`self.K2_AddActorWorldOffset` (* (`KismetMathLibrary.Normal` _returnvalue) (`KismetMathLibrary.FMin` (`KismetMathLibrary.VSize` _returnvalue) (* DeltaSeconds (`self.MoveSpeed`))))))

(event `Move`
  (params (Location :type "Vector Structure"))
  (set `self.NextPos` Location))

(fn `UserConstructionScript`
  (bind _p_player1_marker (`self.P_player1_marker`))
  (if (`self.IsPlayer1`)
    (`ParticleSystemComponent.SetTemplate` _p_player1_marker "/Game/FXVarietyPack/Particles/P_player1_marker.P_player1_marker")
    (else
      (`ParticleSystemComponent.SetTemplate` _p_player1_marker "/Game/FXVarietyPack/Particles/P_player2_marker.P_player2_marker"))))