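; BP_Rotcore is an actor that spawns and drives two BP_UVText labels, apparently for the UV light feature.
; On BeginPlay it spawns one at each of two scene components and sets their text from two variables.
; After a five-second delay it switches the first label's material to M_UVText_2.
; Tick keeps that first label matched to its component's world location and rotation, while the second stays where spawned.
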(event `self.ReceiveBeginPlay`
  (bind _returnvalue (`|SpawnActorFromClass` "/Game/UVLight/Blueprints/BP_UVText.BP_UVText_C" (`KismetMathLibrary.Conv_VectorToTransform` (`SceneComponent.K2_GetComponentLocation` (`self.Scene`))) "Undefined" "OverrideRootScale" null null))
  (`TextRenderComponent.K2_SetText` (`/Game/UVLight/Blueprints/BP_UVText.TextRender` _returnvalue) (`self.NewVar_0`))
  (set `self.NewVar_2` _returnvalue)
  (bind _returnvalue_2 (`|SpawnActorFromClass` "/Game/UVLight/Blueprints/BP_UVText.BP_UVText_C" (`KismetMathLibrary.Conv_VectorToTransform` (`SceneComponent.K2_GetComponentLocation` (`self.Scene1`))) "Undefined" "OverrideRootScale" null null))
  (`TextRenderComponent.K2_SetText` (`/Game/UVLight/Blueprints/BP_UVText.TextRender` _returnvalue_2) (`self.NewVar_1`))
  (`KismetSystemLibrary.Delay` 5.0)
  (`TextRenderComponent.SetTextMaterial` (`/Game/UVLight/Blueprints/BP_UVText.TextRender` (`self.NewVar_2`)) "/Game/UVLight/Materials/M_UVText_2.M_UVText_2"))

(event `self.ReceiveTick`
  (params (DeltaSeconds :type "Float (single-precision)"))
  (bind _scene (`self.Scene`))
  (`self.K2_SetActorLocationAndRotation` (`self.NewVar_2`) (`SceneComponent.K2_GetComponentLocation` _scene) (`SceneComponent.K2_GetComponentRotation` _scene) false false))

(fn `UserConstructionScript`)