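; BP_UVHPBar is a text display whose UV material intensity responds to nearby UV emitters.
; Construction sets the text and detection sphere radius, then builds a dynamic M_UVText material with color, seeded random offset and noise, passing NoiseU and NoiseV crosswise.
; Each tick, CalculateUV sums distance-attenuated strengths from overlapping BI_UVEmit actors into the material's Intensity.
; A direction-weighted vector sum is also accumulated but never affects the output.
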(event `self.ReceiveTick`
  (params (DeltaSeconds :type "Float (single-precision)"))
  (`self.CalculateUV`))

(fn `CalculateUV`
  (locals (StrengthSum :type "Float (double-precision)") (VectorSum :type "Vector Structure"))
  (set `local.StrengthSum` 0.0)
  (bind _output_get (set `local.VectorSum` (0.0 0.0 0.0)))
  (for _array_element (`PrimitiveComponent.GetOverlappingActors` (`self.Sphere`) "/Script/Engine.Actor")
    (if (`KismetSystemLibrary.DoesImplementInterface` _array_element "/Game/UVLight/Blueprints/BI_UVEmit.BI_UVEmit_C")
      (bind (_location _strength) (message `/Game/UVLight/Blueprints/BI_UVEmit.GetUV` _array_element))
      (bind _returnvalue (- _location (`SceneComponent.K2_GetComponentLocation` (`self.TextRender`))))
      (bind _returnvalue_2 (`KismetMathLibrary.VSize` _returnvalue))
      (set `local.StrengthSum` (+ (* (`KismetMathLibrary.MultiplyMultiply_FloatFloat` (- 1.0 (/ _returnvalue_2 (`self.Radius`))) (`self.DistanceExponent`)) _strength) (`local.StrengthSum`)))
      (set `local.VectorSum` (+ (`local.VectorSum`) (* (`KismetMathLibrary.Normal` _returnvalue) (- (`self.Radius`) _returnvalue_2))))))
  (`MaterialInstanceDynamic.SetScalarParameterValue` (`self.Material`) "Intensity" (`local.StrengthSum`)))

(fn `UserConstructionScript`
  (`TextRenderComponent.K2_SetText` (`self.TextRender`) (`self.Text`))
  (`SphereComponent.SetSphereRadius` (`self.Sphere`) (`self.Radius`) true)
  (bind _returnvalue (`PrimitiveComponent.CreateDynamicMaterialInstance` (`self.TextRender`) 0 "/Game/UVLight/Materials/M_UVText.M_UVText" "None"))
  (bind _output_get (set `self.Material` _returnvalue))
  (`MaterialInstanceDynamic.SetScalarParameterValue` _output_get "RandomOffset" (`KismetMathLibrary.RandomFloatFromStream` (`self.RandomSeed`)))
  (`MaterialInstanceDynamic.SetVectorParameterValue` (`self.Material`) "Color" (`self.Color`))
  (`MaterialInstanceDynamic.SetScalarParameterValue` (`self.Material`) "NoisePow" (`self.NoisePow`))
  (`MaterialInstanceDynamic.SetScalarParameterValue` (`self.Material`) "NoiseU" (`self.NoiseV`))
  (`MaterialInstanceDynamic.SetScalarParameterValue` (`self.Material`) "NoiseV" (`self.NoiseU`)))