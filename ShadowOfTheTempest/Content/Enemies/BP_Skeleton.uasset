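; Skeleton enemy Blueprint that reacts to overlaps with other actors.
; Overlapping a BP_Doorway in its first enum state sets Health to zero, then runs OnHit; a doorway in any other state is ignored.
; Non-doorway overlaps call OnHit directly.
; When OnHit returns true and Mode is 2, the mesh plays the skeleton damage animation once.
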(event `self.ReceiveActorBeginOverlap`
  (params (OtherActor :type "Actor Object Reference"))
  (bind _asbp_doorway (cast `/Game/Props/BP_Doorway` OtherActor)
    (:`then`
      (if (`|EnumEquality` (`/Game/Props/BP_Doorway.CurrentState` _asbp_doorway) "NewEnumerator0")
        (set `self.Health` 0)
        (bind _shouldnotplayanim (`self.OnHit` OtherActor :!label _label))
        (if _shouldnotplayanim
          (if (== (`self.Mode`) 2)
            (`SkeletalMeshComponent.PlayAnimation` (`self.Mesh`) "/Game/Enemies/Skeleton/Animation/Skeleton_Damage_Anim.Skeleton_Damage_Anim" false)))))
    (:`CastFailed`
      (goto _label))))

(fn `UserConstructionScript`)