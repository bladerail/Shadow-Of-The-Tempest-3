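; BP_EnemyProjectile is an enemy spell projectile that damages the player wizard on contact.
; On spawn it plays a launch sound and a color-tinted shockwave emitter, then destroys itself after its Lifetime delay, while Tick counts down a separate Duration variable.
; A box overlap that casts to BP_Wizard applies Damage through ReceiveDamage, spawns impact effects and sound, and destroys the projectile, ignoring other actors.
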(event `self.ReceiveBeginPlay`
  (bind _defaultsceneroot (`self.DefaultSceneRoot`))
  (bind _returnvalue (`SceneComponent.K2_GetComponentLocation` _defaultsceneroot))
  ;[1 1 1] spawn shot shockwave
  (set `self.Duration` (`self.Lifetime`))
  (bind _returnvalue_2 (`GameplayStatics.SpawnEmitterAtLocation` "/Game/FXVarietyPack/Particles/P_ky_spellShotShockwave.P_ky_spellShotShockwave" _returnvalue (`SceneComponent.K2_GetComponentRotation` _defaultsceneroot) (3.0 3.0 3.0)))
  (`GameplayStatics.PlaySoundAtLocation` "/Game/Enemies/Apparition/Audio/Apparition_Projectile_Launch.Apparition_Projectile_Launch" _returnvalue (struct) 1.0 1.0 0.0 null null null)
  (`ParticleSystemComponent.SetVectorParameter` _returnvalue_2 "color" (`KismetMathLibrary.Conv_LinearColorToVector` (`self.Color`)))
  ;[1 1 1] Destroy projectile after lifetime is over
  (`KismetSystemLibrary.Delay` (`self.Lifetime`))
  (`self.K2_DestroyActor`))

(event `self.ReceiveTick`
  (params (DeltaSeconds :type "Float (single-precision)"))
  ;[1 1 1] Duration decrement for control
  (set `self.duration` (- (`self.duration`) DeltaSeconds)))

(event `self.Box.OnComponentBeginOverlap`
  (params (OverlappedComponent :type "PrimitiveComponent Object Reference") (OtherActor :type "Actor Object Reference") (OtherComp :type "PrimitiveComponent Object Reference") (OtherBodyIndex :type Integer) (bFromSweep :type Boolean) (SweepResult :type "HitResult Structure (by ref)"))
  (bind _returnvalue (`SceneComponent.K2_GetComponentLocation` (`self.SpellProjectile`)))
  ;[1 1 1] Spawn FX and sound when projectile hit player
  (bind _asbp_wizard (cast `/Game/Players/BP_Wizard` OtherActor))
  (`/Game/Enemies/BP_EnemyAttackable.ReceiveDamage` _asbp_wizard (`self.Damage`))
  (`GameplayStatics.SpawnEmitterAtLocation` (`self.SpellHitFx`) _returnvalue)
  (`GameplayStatics.PlaySoundAtLocation` "/Game/Players/Audio/Player_SpellImpact.Player_SpellImpact" _returnvalue (struct) 1.0 1.0 0.0 null null null)
  (`self.K2_DestroyActor`))

(fn `UserConstructionScript`)