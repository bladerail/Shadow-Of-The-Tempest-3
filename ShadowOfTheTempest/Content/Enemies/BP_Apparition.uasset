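; Apparition enemy that fires projectiles and extends its parent's hit handling.
; AttackEffect spawns an enemy projectile slightly above the actor, along its facing.
; On overlap, OnHit zeroes health for a doorway in its first state, and passes simple projectiles to the parent only when they touch the Box hitbox, otherwise flagging a miss through a server event.
; A true hit result in Mode 2 plays the damage animation.
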(event `self.ReceiveActorBeginOverlap`
  (params (OtherActor :type "Actor Object Reference"))
  (bind _shouldnotplayanim (`self.OnHit` OtherActor))
  (if _shouldnotplayanim
    (if (== (`self.Mode`) 2)
      (`SkeletalMeshComponent.PlayAnimation` (`self.Mesh`) "/Game/Enemies/Apparition/Animation/Apparition_Damage_Anim.Apparition_Damage_Anim" false))))

(event `self.AttackEffect`
  (`|SpawnActorFromClass` "/Game/Enemies/BP_EnemyProjectile.BP_EnemyProjectile_C" (`KismetMathLibrary.MakeTransform` (+ (`self.K2_GetActorLocation`) (0.0 0.0 50.0)) (`self.K2_GetActorRotation`)) "Undefined" "OverrideRootScale" null null))

(event `Server Miss Hitbox`
  (params (`Target projectile` :type "/Game/Players/BP_SimpleProjectile Object Reference"))
  (`/Game/Players/BP_SimpleProjectile.MissHitbox` `Target projectile`))

(event `Server Destroy Apparition`
  (params (`Destroy Target` :type "Actor Object Reference"))
  (`self.K2_DestroyActor` `Destroy Target`))

(fn `OnHit`
  (params (Object :type "Actor Object Reference"))
  (returns (ShouldNotPlayAnim :type Boolean))
  (bind _asbp_doorway (cast `/Game/Props/BP_Doorway` Object)
    (:`then`
      (if (`|EnumEquality` (`/Game/Props/BP_Doorway.CurrentState` _asbp_doorway) "NewEnumerator0")
        (set `self.Health` 0)
        (bind _shouldnotplayanim (`parent.OnHit` Object :!label _label))
        (return _shouldnotplayanim)))
    (:`CastFailed`
      (bind _asbp_simple_projectile (cast `/Game/Players/BP_SimpleProjectile` Object)
        (:`then`
          (if (`PrimitiveComponent.IsOverlappingComponent` (`/Game/Players/BP_SimpleProjectile.Capsule` _asbp_simple_projectile) (`self.Box`))
            (goto _label)
            (else
              (`self.Server Miss Hitbox` _asbp_simple_projectile)
              (return true))))
        (:`CastFailed`
          (return true))))))

(fn `UserConstructionScript`)