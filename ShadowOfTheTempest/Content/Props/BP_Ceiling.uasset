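; BP_Ceiling is a prop actor that builds a ceiling as a grid of repeated mesh tiles.
; Its construction script loops over Length and Width, placing one instanced static mesh per cell at the sum of the index-scaled LengthOffset and WidthOffset, with no rotation and unit scale.
; The event graph holds only disabled placeholder events, so it has no runtime logic.
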(fn `UserConstructionScript`
  (for _index (range (`self.Length`))
    (for _index_2 (range (`self.Width`))
      (`InstancedStaticMeshComponent.AddInstance` (`self.InstancedStaticMesh`) (`KismetMathLibrary.MakeTransform` (+ (* (`self.Length_Offset`) _index) (* (`self.Width_Offset`) _index_2)))))))