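; Doorway prop with a portcullis that falls or rises, which the Wind Wizard's spell can act on.
; Tick offsets the gate by CurrentSpeed, turns winches from its height and stops near either endpoint, starting an optional Boss once fully raised.
; CastSpell and DeactivateSpell delegate to BP_WindWizard; client/server events set or reset speed.
; A leaf vortex shows while the fall speed is altered, and audio follows movement and spell hold.
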(event `self.ReceiveBeginPlay`
  ;[1 1 1] Set original Speed and play sound if already falling
  (set `self.CurrentSpeed` (`self.OriginalSpeed`))
  (if (`|EnumEquality` (`self.CurrentState`) "NewEnumerator0")
    (`AudioComponent.Play` (`self.PortcullisMovingAudio`) 0.0)))

(event `self.ReceiveTick`
  (params (DeltaSeconds :type "Float (single-precision)"))
  (bind _boss (`self.Boss`))
  (bind _portcullis (`self.Portcullis`))
  (bind _currentstate (`self.CurrentState`))
  (bind _portcullis_2 (`self.Portcullis`))
  (bind _returnvalue_location (`KismetMathLibrary.BreakTransform` (`SceneComponent.GetRelativeTransform` (`self.Portcullis`))))
  (if (`KismetSystemLibrary.IsValid` (`self.Portcullis`))
    (`|ExecutionSequence`
      (:`then_0`
        (switch `/Game/Props/BP_DoorwayStates` _currentstate
          (:`NewEnumerator0`
            _)
          (:`NewEnumerator2`
            _))
        (for _array_element (`self.Winch`)
          (`/Game/BP_Winch.Rotate` _array_element (.z _returnvalue_location))))
      (:`then_1`
        (switch `/Game/Props/BP_DoorwayStates` _currentstate
          (:`NewEnumerator0`
            ;[1 1 1] Falling
            (if (== (`self.CurrentSpeed`) (`self.OriginalSpeed`))
              (`ActorComponent.SetActive` (`self.P_Leaves_Vortex`) false false)
              (else
                (`ActorComponent.SetActive` (`self.P_Leaves_Vortex`) true false)))
            (`SceneComponent.K2_AddLocalOffset` _portcullis_2 (* (`KismetMathLibrary.MakeVector` 0.0 0.0 (`self.CurrentSpeed`)) DeltaSeconds) false false)
            (if (<= (- (.z (`SceneComponent.RelativeLocation` _portcullis_2)) (.z (`self.EndPoint`))) 10.0)
              (set `self.CurrentState` "NewEnumerator1")
              (`ActorComponent.SetActive` (`self.P_Leaves_Vortex`) false false)
              (`GameplayStatics.PlaySoundAtLocation` "/Game/Players/Audio/Wind_PortculisClosed.Wind_PortculisClosed" (`SceneComponent.K2_GetComponentLocation` (`self.Portcullis`)) (struct) 1.0 1.0 0.0 null null null)
              (`AudioComponent.Stop` (`self.PortcullisMovingAudio`))))
          (:`NewEnumerator2`
            ;[1 1 1] Rising
            (`SceneComponent.K2_AddLocalOffset` _portcullis (* (`KismetMathLibrary.MakeVector` 0.0 0.0 (* (`self.CurrentSpeed`) -0.6)) DeltaSeconds) false false)
            (if (<= (- (.z (`self.StartPoint`)) (.z (`SceneComponent.RelativeLocation` _portcullis))) 10.0)
              (set `self.CurrentState` "NewEnumerator1")
              (`/Engine/EditorBlueprintResources/StandardMacros.IsValid` _boss
                (:`Is Valid`
                  (`/Game/BP_Boss.Start` _boss))
                (:`Is Not Valid`
                  _))
              (`AudioComponent.Stop` (`self.PortcullisMovingAudio`)))))))))

(event `/Game/Players/Spells/BP_Spell_Interface.CastSpell`
  (params (CastPoint :type "Vector Structure") (Strength :type "Float (single-precision)") (ContactPoint :type "Vector Structure"))
  ;[1 1 1] Wind Wizard Cast Portcullis Spell
  (bind _outactors (`GameplayStatics.GetAllActorsOfClass` "/Game/Players/BP_WindWizard.BP_WindWizard_C"))
  (`/Game/Players/BP_WindWizard.Wind Cast Portcullis` (`|GetArrayItem` _outactors) Strength self)
  (`AudioComponent.Play` (`self.PortcullisHoldAudio`) 0.0))

(event `Client Set Current Speed`
  (params (Speed :type "Float (double-precision)"))
  (`self.Server Set Current Speed` Speed))

(event `Client Deactivate`
  (set `self.CurrentSpeed` (`self.OriginalSpeed`) :!label _label)
  (`ActorComponent.SetActive` (`self.P_Leaves_Vortex`) false false))

(event `/Game/Players/Spells/BP_Spell_Interface.DeactivateSpell`
  ;[1 1 1] Deactivate Portcullis Spell
  (bind _outactors (`GameplayStatics.GetAllActorsOfClass` "/Game/Players/BP_WindWizard.BP_WindWizard_C"))
  (`/Game/Players/BP_WindWizard.Wind Deactivate Portcullis` (`|GetArrayItem` _outactors) self (`self.P_Leaves_Vortex`))
  (`AudioComponent.Stop` (`self.PortcullisHoldAudio`)))

(event `Server Set Current Speed`
  (params (Speed :type "Float (double-precision)"))
  (set `self.CurrentSpeed` Speed))

(event `Server Deactivate`
  (goto _label))

(event `InputAction|Reset`
  (params (Key :type "Key Structure")))

(event `BeginFall`
  (bind _portcullismovingaudio (`self.PortcullisMovingAudio`))
  ;[1 1 1] Event to start falling
  (if (not (<= (- (.z (`SceneComponent.RelativeLocation` (`self.Portcullis`))) (.z (`self.EndPoint`))) 10.0))
    (set `self.CurrentState` "NewEnumerator0")
    (`AudioComponent.SetSound` _portcullismovingaudio "/Game/Players/Audio/Wind_PortculisFalling.Wind_PortculisFalling")
    (`AudioComponent.Play` _portcullismovingaudio 0.0)))

(event `Raise`
  (bind _portcullismovingaudio (`self.PortcullisMovingAudio`))
  ;[1 1 1] Event to start raising Portcullis
  (if (not (<= (- (.z (`self.StartPoint`)) (.z (`SceneComponent.RelativeLocation` (`self.Portcullis`)))) 10.0))
    (`/Game/Players/Spells/BP_Spell_Interface.DeactivateSpell`)
    (set `self.CurrentState` "NewEnumerator2")
    (`AudioComponent.SetSound` _portcullismovingaudio "/Game/Players/Audio/Wind_PortculisRaising.Wind_PortculisRaising")
    (`AudioComponent.Play` _portcullismovingaudio 0.0)
    (bind _outactors (`GameplayStatics.GetAllActorsOfClass` "/Game/Players/BP_WindWizard.BP_WindWizard_C"))
    (bind _output (`|GetArrayItem` _outactors))
    (if (== (`/Game/Players/BP_Wizard.ActiveSpellOnMap` _output) self)
      (`/Game/Players/BP_Wizard.SetNewActiveSpell` _output null))))

(fn `Destroy`
  (`ActorComponent.K2_DestroyComponent` (`self.Portcullis`)))

(fn `UserConstructionScript`)