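; BP_GlobalLight is a lighting prop that groups five directional lights under a single strength setting.
; Its construction script applies the LightStrength variable as the intensity of all five lights, so they always share one brightness value.
; The event graph holds only disabled placeholder events, so the Blueprint adds no runtime logic.
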(fn `UserConstructionScript`
  (bind _light_strength (`self.Light_Strength`))
  (`LightComponent.SetIntensity` (`self.DirectionalLight`) _light_strength)
  (`LightComponent.SetIntensity` (`self.DirectionalLight1`) _light_strength)
  (`LightComponent.SetIntensity` (`self.DirectionalLight2`) _light_strength)
  (`LightComponent.SetIntensity` (`self.DirectionalLight3`) _light_strength)
  (`LightComponent.SetIntensity` (`self.DirectionalLight4`) _light_strength))