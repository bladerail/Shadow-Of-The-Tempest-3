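; A pressure board prop that raises a linked BP_Doorway when a BP_Wizard steps on it.
; PlayerDetect overlaps flip a two-value State, play a press or release sound and animate BoardMesh's Z through timelines.
; The doorway's Raise fires only when the press timeline finishes.
; Release reverses a separate timeline to move the board and sends nothing to the doorway.
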(event `self.PlayerDetect.OnComponentBeginOverlap`
  (params (OverlappedComponent :type "PrimitiveComponent Object Reference") (OtherActor :type "Actor Object Reference") (OtherComp :type "PrimitiveComponent Object Reference") (OtherBodyIndex :type Integer) (bFromSweep :type Boolean) (SweepResult :type "HitResult Structure (by ref)"))
  (cast `/Game/Players/BP_Wizard` OtherActor)
  (if (== (`self.State`) 0)
    (set `self.State` 1)
    (`GameplayStatics.PlaySoundAtLocation` "/Game/Players/Audio/PressurePlate_Triggered.PressurePlate_Triggered" (`self.K2_GetActorLocation`) (struct) 1.0 1.0 0.0 null null null)
    (bind (_direction _down) (`Timeline|Timeline_down` :!via `PlayFromStart`)
      (:`Update`
        (`SceneComponent.K2_SetRelativeLocation` (`self.BoardMesh`) (`KismetMathLibrary.MakeVector` 0.0 0.0 _down) false false))
      (:`Finished`
        (bind _asbp_doorway (cast `/Game/Props/BP_Doorway` (`self.Doorway`)))
        (`/Game/Props/BP_Doorway.Raise` _asbp_doorway)))))

(event `self.PlayerDetect.OnComponentEndOverlap`
  (params (OverlappedComponent :type "PrimitiveComponent Object Reference") (OtherActor :type "Actor Object Reference") (OtherComp :type "PrimitiveComponent Object Reference") (OtherBodyIndex :type Integer))
  (cast `/Game/Players/BP_Wizard` OtherActor)
  (if (== (`self.State`) 1)
    (set `self.State` 0)
    (`GameplayStatics.PlaySoundAtLocation` "/Game/Players/Audio/PressurePlate_Released.PressurePlate_Released" (`self.K2_GetActorLocation`) (struct) 1.0 1.0 0.0 null null null)
    (bind (_direction _down) (`Timeline|Timeline_0` :!via `ReverseFromEnd`)
      (:`Update`
        (`SceneComponent.K2_SetRelativeLocation` (`self.BoardMesh`) (`KismetMathLibrary.MakeVector` 0.0 0.0 _down) false false)))))

(fn `UserConstructionScript`)